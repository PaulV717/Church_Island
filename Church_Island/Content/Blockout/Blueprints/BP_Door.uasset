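; Configurable blockout door, single or double, that swings open when its box volume is overlapped and closes when overlap ends, unless locked or non-movable.
; The construction script sets up meshes, materials, mobility and volume size from frame bounds, and previews open angles, also applied to static doors.
; A timeline scaled by opening time lerps yaw from the captured current angle, while paired DoOnce gates alternate opening and closing.
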(event OnComponentBeginOverlap(CharacterOverlapVolume)
  (params (OverlappedComponent :type Primitive%20Component%20Object%20Reference) (OtherActor :type Actor%20Object%20Reference) (OtherComp :type Primitive%20Component%20Object%20Reference) (OtherBodyIndex :type Integer) (bFromSweep :type Boolean) (SweepResult :type Hit%20Result%20Structure%20%28by%20ref%29))
  (if (Utilities|Enum|Equal(Enum) (Variables|Default|GetDoors%20Mobility) "Movable")
    (if (not (Variables|Default|GetIs%20Door%20Locked?))
      (Utilities|FlowControl|Sequence
        (:then_0
          (Utilities|FlowControl|DoOnce false
            (:Completed
              (Utilities|FlowControl|Sequence
                (:then_0
                  (bind (_direction _0_1) (Timeline|Animate%20Door%20Open-Closed Stop)
                    (:Update
                      (Transformation|SetRelativeRotation (Variables|Default|GetSM_Door%201) (Math|Rotator|MakeRotator 0.0 0.0 (Utilities|Select :Index _direction :Forward (Math|Float|Lerp (Variables|Values|GetStarting%20Position%20-%20Door%201) (Variables|Default|GetDoor%201%20-%20Open%20Angle) _0_1) :Backward (Math|Float|Lerp 0.0 (Variables|Values|GetStarting%20Position%20-%20Door%201) _0_1))) false false)
                      (if (Variables|Default|GetIs%20this%20a%20double%20door?)
                        (Transformation|SetRelativeRotation (Variables|Default|GetSM_Door%202) (Math|Rotator|MakeRotator 0.0 0.0 (Utilities|Select :Index _direction :Forward (Math|Float|Lerp (Variables|Values|GetStarting%20Position%20-%20Door%202) (* (Variables|Default|GetDoor%202%20-%20Open%20Angle) -1.0) _0_1) :Backward (Math|Float|Lerp 0.0 (Variables|Values|GetStarting%20Position%20-%20Door%202) _0_1))) false false)))))
                (:then_1
                  (Variables|Values|SetStarting%20Position%20-%20Door%201 (.yaw (Variables|/Script/Engine.SceneComponent|GetRelativeRotation (Variables|Default|GetSM_Door%201))))
                  (if (Variables|Default|GetIs%20this%20a%20double%20door?)
                    (Variables|Values|SetStarting%20Position%20-%20Door%202 (.yaw (Variables|/Script/Engine.SceneComponent|GetRelativeRotation (Variables|Default|GetSM_Door%202))))
                    (Timeline|Animate%20Door%20Open-Closed PlayFromStart)
                    (else
                      (Timeline|Animate%20Door%20Open-Closed PlayFromStart))))))))
        (:then_1
          (Utilities|FlowControl|DoOnce false) ; enters at Reset
        )))))

(event OnComponentEndOverlap(CharacterOverlapVolume)
  (params (OverlappedComponent :type Primitive%20Component%20Object%20Reference) (OtherActor :type Actor%20Object%20Reference) (OtherComp :type Primitive%20Component%20Object%20Reference) (OtherBodyIndex :type Integer))
  (if (Utilities|Enum|Equal(Enum) (Variables|Default|GetDoors%20Mobility) "Movable")
    (if (not (Variables|Default|GetIs%20Door%20Locked?))
      (Utilities|FlowControl|Sequence
        (:then_0
          (Utilities|FlowControl|DoOnce false
            (:Completed
              (Utilities|FlowControl|Sequence
                (:then_0
                  (bind (_direction _0_1) (Timeline|Animate%20Door%20Open-Closed Stop)
                    (:Update
                      (Transformation|SetRelativeRotation (Variables|Default|GetSM_Door%201) (Math|Rotator|MakeRotator 0.0 0.0 (Utilities|Select :Index _direction :Forward (Math|Float|Lerp (Variables|Values|GetStarting%20Position%20-%20Door%201) (Variables|Default|GetDoor%201%20-%20Open%20Angle) _0_1) :Backward (Math|Float|Lerp 0.0 (Variables|Values|GetStarting%20Position%20-%20Door%201) _0_1))) false false)
                      (if (Variables|Default|GetIs%20this%20a%20double%20door?)
                        (Transformation|SetRelativeRotation (Variables|Default|GetSM_Door%202) (Math|Rotator|MakeRotator 0.0 0.0 (Utilities|Select :Index _direction :Forward (Math|Float|Lerp (Variables|Values|GetStarting%20Position%20-%20Door%202) (* (Variables|Default|GetDoor%202%20-%20Open%20Angle) -1.0) _0_1) :Backward (Math|Float|Lerp 0.0 (Variables|Values|GetStarting%20Position%20-%20Door%202) _0_1))) false false)))))
                (:then_1
                  (Variables|Values|SetStarting%20Position%20-%20Door%201 (.yaw (Variables|/Script/Engine.SceneComponent|GetRelativeRotation (Variables|Default|GetSM_Door%201))))
                  (if (Variables|Default|GetIs%20this%20a%20double%20door?)
                    (Variables|Values|SetStarting%20Position%20-%20Door%202 (.yaw (Variables|/Script/Engine.SceneComponent|GetRelativeRotation (Variables|Default|GetSM_Door%202))))
                    (Timeline|Animate%20Door%20Open-Closed ReverseFromEnd)
                    (else
                      (Timeline|Animate%20Door%20Open-Closed ReverseFromEnd))))))))
        (:then_1
          (Utilities|FlowControl|DoOnce false) ; enters at Reset
        )))))

(event EventBeginPlay
  (Components|Timeline|SetPlayRate (Variables|Default|GetAnimate%20Door%20Open-Closed) (/ 1.0 (Variables|Default|GetDoor%20Opening%20Time)))
  (if (Utilities|Enum|Equal(Enum) (Variables|Default|GetDoors%20Mobility) "Movable")
    (if (Variables|Default|GetStart%20Colsed%20when%20game%20plays?)
      (Transformation|SetRelativeRotation (Variables|Default|GetSM_Door%201) (Math|Rotator|MakeRotator 0.0 0.0 0.0) false false)
      (if (Variables|Default|GetIs%20this%20a%20double%20door?)
        (Transformation|SetRelativeRotation (Variables|Default|GetSM_Door%202) (Math|Rotator|MakeRotator 0.0 0.0 0.0) false false)))))

(fn ConstructionScript
  (bind _new_door_geometry_2 (Variables|Default|GetNew%20Door%20Geometry%202))
  (bind _door_material (Variables|Default|GetDoor%20Material))
  (bind _sm_doorframe (Variables|Default|GetSM_Doorframe))
  (bind _collision_overlap_scale (Variables|Default|GetCollision%20overlap%20Scale))
  (bind _frame_material (Variables|Default|GetFrame%20Material))
  (bind _door_material_2 (Variables|Default|GetDoor%20Material))
  (bind _new_door_geometry_1 (Variables|Default|GetNew%20Door%20Geometry%201))
  (bind _sm_doorframe_2 (Variables|Default|GetSM_Doorframe))
  (bind _collision_overlap_scale_2 (Variables|Default|GetCollision%20overlap%20Scale))
  (bind _new_door_geometry_1_2 (Variables|Default|GetNew%20Door%20Geometry%201))
  (bind _frame_material_2 (Variables|Default|GetFrame%20Material))
  (bind _new_doorframe_geometry (Variables|Default|GetNew%20Doorframe%20Geometry))
  (bind _new_doorframe_geometry_2 (Variables|Default|GetNew%20Doorframe%20Geometry))
  (bind _max (Components|StaticMesh|GetLocalBounds _sm_doorframe))
  (bind _max_2 (Components|StaticMesh|GetLocalBounds _sm_doorframe_2))
  (bind _returnvalue (+ (.z _collision_overlap_scale) (.z _max)))
  (bind _returnvalue_2 (+ (.z _collision_overlap_scale_2) (.z _max_2)))
  (bind _returnvalue_3 (* _returnvalue 0.5))
  (bind _returnvalue_4 (* _returnvalue_2 0.5))
  (if (Variables|Default|GetIs%20this%20a%20double%20door?)
    (Transformation|SetRelativeLocation (Variables|Default|GetSM_Door%201) "9.523272,107.485146,0.000000" false true)
    (Transformation|SetRelativeLocation (Variables|Default|GetSM_Door%202) "9.523272,-107.485146,0.000000" false true)
    (Components|StaticMesh|SetStaticMesh (Variables|Default|GetSM_Doorframe) "/Game/Blockout/Geometry/Assets/Doors/SM_Doorframe_Double.SM_Doorframe_Double")
    (Components|StaticMesh|SetStaticMesh (Variables|Default|GetSM_Door%201) "/Game/Blockout/Geometry/Assets/Doors/SM_Door1_Double_Left.SM_Door1_Double_Left")
    (Components|Box|SetBoxExtent (Variables|Default|GetCharacter%20Overlap%20Volume) (Math|Vector|MakeVector (.x _collision_overlap_scale) (+ (.y _collision_overlap_scale) (.y _max)) _returnvalue_3) true)
    (Transformation|SetRelativeTransform (Variables|Default|GetCharacter%20Overlap%20Volume) (Math|Transform|MakeTransform (Math|Vector|MakeVector 0.0 0.0 _returnvalue_3) "0, 0, 0" "1,1,1") false true)
    (Transformation|SetMobility (Variables|Default|GetSM_Door%201) (Variables|Default|GetDoors%20Mobility))
    (if (Variables|Default|GetUse%20Doorframe?)
      (Utilities|IsValid _new_doorframe_geometry_2
        (:Is%20Valid
          (Components|StaticMesh|SetStaticMesh (Variables|Default|GetSM_Doorframe) _new_doorframe_geometry_2))
        (:Is%20Not%20Valid
          _))
      (Utilities|IsValid _frame_material_2
        (:Is%20Valid
          (Rendering|Material|SetMaterial (Variables|Default|GetSM_Doorframe) (Variables|Default|GetFrame%20Material%20ID) _frame_material_2))
        (:Is%20Not%20Valid
          _))
      (else
        (Components|DestroyComponent (Variables|Default|GetSM_Doorframe))))
    (Utilities|IsValid _new_door_geometry_1_2
      (:Is%20Valid
        (Components|StaticMesh|SetStaticMesh (Variables|Default|GetSM_Door%201) _new_door_geometry_1_2))
      (:Is%20Not%20Valid
        _))
    (Utilities|IsValid _new_door_geometry_2
      (:Is%20Valid
        (Components|StaticMesh|SetStaticMesh (Variables|Default|GetSM_Door%202) _new_door_geometry_2))
      (:Is%20Not%20Valid
        _))
    (Utilities|IsValid _door_material
      (:Is%20Valid
        (Rendering|Material|SetMaterial (Variables|Default|GetSM_Door%201) (Variables|Default|GetDoor%20Material%20ID) _door_material))
      (:Is%20Not%20Valid
        _))
    (if (Variables|Default|GetPreview%20Doors%20Open%20Angles?)
      (Transformation|SetRelativeRotation (Variables|Default|GetSM_Door%201) (Math|Rotator|MakeRotator 0.0 0.0 (Variables|Default|GetDoor%201%20-%20Open%20Angle)) false false :!label _label)
      (Transformation|SetRelativeRotation (Variables|Default|GetSM_Door%202) (Math|Rotator|MakeRotator 0.0 0.0 (* (Variables|Default|GetDoor%202%20-%20Open%20Angle) -1.0)) false false)
      (elif (Utilities|Enum|Equal(Enum) (Variables|Default|GetDoors%20Mobility) "Static")
        (goto _label)))
    (else
      (Transformation|SetRelativeLocation (Variables|Default|GetSM_Door%201) "9.523272,57.431908,0.000000" false true)
      (Components|DestroyComponent (Variables|Default|GetSM_Door%202))
      (Components|Box|SetBoxExtent (Variables|Default|GetCharacter%20Overlap%20Volume) (Math|Vector|MakeVector (.x _collision_overlap_scale_2) (+ (.y _collision_overlap_scale_2) (.y _max_2)) _returnvalue_4) true)
      (Transformation|SetRelativeTransform (Variables|Default|GetCharacter%20Overlap%20Volume) (Math|Transform|MakeTransform (Math|Vector|MakeVector 0.0 0.0 _returnvalue_4) "0, 0, 0" "1,1,1") false true)
      (Transformation|SetMobility (Variables|Default|GetSM_Door%201) (Variables|Default|GetDoors%20Mobility))
      (if (Variables|Default|GetUse%20Doorframe?)
        (Utilities|IsValid _new_doorframe_geometry
          (:Is%20Valid
            (Components|StaticMesh|SetStaticMesh (Variables|Default|GetSM_Doorframe) _new_doorframe_geometry))
          (:Is%20Not%20Valid
            _))
        (Utilities|IsValid _frame_material
          (:Is%20Valid
            (Rendering|Material|SetMaterial (Variables|Default|GetSM_Doorframe) (Variables|Default|GetFrame%20Material%20ID) _frame_material))
          (:Is%20Not%20Valid
            _))
        (else
          (Components|DestroyComponent (Variables|Default|GetSM_Doorframe))))
      (Utilities|IsValid _new_door_geometry_1
        (:Is%20Valid
          (Components|StaticMesh|SetStaticMesh (Variables|Default|GetSM_Door%201) _new_door_geometry_1))
        (:Is%20Not%20Valid
          _))
      (Utilities|IsValid _door_material_2
        (:Is%20Valid
          (Rendering|Material|SetMaterial (Variables|Default|GetSM_Door%201) (Variables|Default|GetDoor%20Material%20ID) _door_material_2))
        (:Is%20Not%20Valid
          _))
      (if (Variables|Default|GetPreview%20Doors%20Open%20Angles?)
        (Transformation|SetRelativeRotation (Variables|Default|GetSM_Door%201) (Math|Rotator|MakeRotator 0.0 0.0 (Variables|Default|GetDoor%201%20-%20Open%20Angle)) false false :!label _label_2)
        (elif (Utilities|Enum|Equal(Enum) (Variables|Default|GetDoors%20Mobility) "Static")
          (goto _label_2))))))
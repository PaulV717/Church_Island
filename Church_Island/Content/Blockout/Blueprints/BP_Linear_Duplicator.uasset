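; Blockout tool that repeats a main mesh in straight runs between editable destination points, such as for walls or fences, optionally closing the loop.
; The construction script fits copies per segment from mesh X bounds plus added length, aimed by look-at rotation.
; Optional scaling spreads leftover distance across copies to reach each point.
; An optional connecting mesh marks joints and the final point, with tinted debug or custom materials.
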(event EventBeginPlay)

(event Collision|EventActorBeginOverlap
  (params (OtherActor :type Actor%20Object%20Reference)))

(event EventTick
  (params (DeltaSeconds :type Float%20%28single-precision%29)))

(fn ConstructionScript
  (bind _main_asset (Variables|Default|GetMain%20Asset))
  (bind _destination_points (Variables|Default|GetDestination%20Points))
  (bind _custom_main_asset_material (Variables|Material|GetCustom%20Main%20Asset%20Material))
  (bind _add_distance_to_asset_length (Variables|Default|GetAdd%20distance%20to%20Asset%20Length))
  (bind _destination_points_2 (Variables|Default|GetDestination%20Points))
  (bind _main_asset_2 (Variables|Default|GetMain%20Asset))
  (bind _unique_colour_for_top_ (Variables|Material|GetUnique%20colour%20for%20top?))
  (bind _custom_connecting_asset_material (Variables|Material|GetCustom%20Connecting%20Asset%20Material))
  (bind _custom_connecting_asset_material_2 (Variables|Material|GetCustom%20Connecting%20Asset%20Material))
  (bind _destination_points_3 (Variables|Default|GetDestination%20Points))
  (bind _returnvalue (Utilities|Array|Length _destination_points_3))
  (bind _returnvalue_2 (Utilities|Array|Length _destination_points_2))
  (bind _returnvalue_3 (StaticMesh|GetBoundingBox _main_asset))
  (bind _returnvalue_4 (StaticMesh|GetBoundingBox _main_asset_2))
  (bind _returnvalue_5 (Math|Conversions|ToFloat(Boolean) _unique_colour_for_top_))
  (bind _returnvalue_6 (- _returnvalue 1))
  (bind _returnvalue_7 (- (.x (.max _returnvalue_4)) (.x (.min _returnvalue_4))))
  (bind _returnvalue_8 (- _returnvalue_2 1))
  (bind _returnvalue_9 (+ _returnvalue_7 _add_distance_to_asset_length))
  (bind _output (Utilities|Array|Get(acopy) _destination_points_2 _returnvalue_8))
  (if (Variables|Material|GetUse%20Debug%20Material?)
    (bind _returnvalue_10 (Rendering|Material|CreateDynamicMaterialInstance "/Game/Blockout/Material/Base/M_WorldProject.M_WorldProject" "None" :!class /Script/Engine.KismetMaterialLibrary))
    (bind _output_get (Variables|Variables|SetMain%20Asset%20Material _returnvalue_10))
    (Rendering|Material|SetVectorParameterValue _output_get "Diffuse Colour" (Variables|Material|GetMain%20Asset%20Colour) :!class /Script/Engine.MaterialInstanceDynamic)
    (Rendering|Material|SetScalarParameterValue _output_get "Roughness" (Variables|Material|GetMaterial%20Roughness%20Value) :!class /Script/Engine.MaterialInstanceDynamic)
    (Rendering|Material|SetScalarParameterValue _output_get "Unique colour for top?" _returnvalue_5 :!class /Script/Engine.MaterialInstanceDynamic)
    (bind _returnvalue_11 (Rendering|Material|CreateDynamicMaterialInstance "/Game/Blockout/Material/Base/M_WorldProject.M_WorldProject" "None" :!class /Script/Engine.KismetMaterialLibrary))
    (bind _output_get_2 (Variables|Variables|SetConnecting%20Asset%20Material _returnvalue_11))
    (Rendering|Material|SetVectorParameterValue _output_get_2 "Diffuse Colour" (Variables|Material|GetConnecting%20Asset%20Colour) :!class /Script/Engine.MaterialInstanceDynamic)
    (Rendering|Material|SetScalarParameterValue _output_get_2 "Roughness" (Variables|Material|GetMaterial%20Roughness%20Value) :!class /Script/Engine.MaterialInstanceDynamic)
    (Rendering|Material|SetScalarParameterValue _output_get_2 "Unique colour for top?" _returnvalue_5 :!class /Script/Engine.MaterialInstanceDynamic))
  (if (> _returnvalue 1)
    (if (Math|Vector|Equal(Vector) (.location (Utilities|Array|Get(acopy) _destination_points _returnvalue_6)) "0, 0, 0" 0.001)
      (Utilities|Array|SetArrayElem (Variables|Default|GetDestination%20Points) _returnvalue_6 (Math|Transform|MakeTransform (+ (.location (Utilities|Array|Get(acopy) _destination_points (- _returnvalue 2))) "100.000000, 0, 0") "0, 0, 0" "1,1,1"))))
  (for (_array_element _array_index) (Variables|Default|GetDestination%20Points)
    (if (== 0 _array_index)
      (if (Variables|Default|GetClose%20Loop?)
        (for _index (range 0 (Math|Integer|Clamp(Integer) (- (Math|Float|Floor (/ (Math|Vector|VectorLength (- (.location (Utilities|Array|Get(acopy) (Variables|Default|GetDestination%20Points) (select (select (== _array_index 0) (Variables|Default|GetClose%20Loop?) false) (- (Utilities|Array|Length (Variables|Default|GetDestination%20Points)) 1) (- _array_index 1)))) (.location _array_element))) _returnvalue_9)) 1) 0 (- (Math|Float|Floor (/ (Math|Vector|VectorLength (- (.location (Utilities|Array|Get(acopy) (Variables|Default|GetDestination%20Points) (select (select (== _array_index 0) (Variables|Default|GetClose%20Loop?) false) (- (Utilities|Array|Length (Variables|Default|GetDestination%20Points)) 1) (- _array_index 1)))) (.location _array_element))) _returnvalue_9)) 1))) :!label _label
          (Utilities|FlowControl|Sequence
            (:then_0
              (Utilities|IsValid (Variables|Default|GetConnecting%20Asset)
                (:Is%20Valid
                  (bind _returnvalue_12 (AddComponent|AddStaticMeshComponent false (Math|Transform|MakeTransform (.location (Utilities|Array|Get(acopy) (Variables|Default|GetDestination%20Points) (select (select (== _array_index 0) (Variables|Default|GetClose%20Loop?) false) (- (Utilities|Array|Length (Variables|Default|GetDestination%20Points)) 1) (- _array_index 1)))) (Math|Rotator|FindLookatRotation (.location (Utilities|Array|Get(acopy) (Variables|Default|GetDestination%20Points) (select (select (== _array_index 0) (Variables|Default|GetClose%20Loop?) false) (- (Utilities|Array|Length (Variables|Default|GetDestination%20Points)) 1) (- _array_index 1)))) (.location (Utilities|Array|Get(acopy) (Variables|Default|GetDestination%20Points) _array_index))) (Math|Vector|MakeVector 1.0 1.0 (Variables|Default|GetHeight)))))
                  (Components|StaticMesh|SetStaticMesh _returnvalue_12 (Variables|Default|GetConnecting%20Asset))
                  (Transformation|AddLocalOffset _returnvalue_12 (Math|Vector|MakeVector (+ (* _index _returnvalue_9) (* _index (select (Variables|Default|GetScale%20assets%20to%20reach%20destination?) (* (/ (- (/ (Math|Vector|VectorLength (- (.location (Utilities|Array|Get(acopy) (Variables|Default|GetDestination%20Points) (select (select (== _array_index 0) (Variables|Default|GetClose%20Loop?) false) (- (Utilities|Array|Length (Variables|Default|GetDestination%20Points)) 1) (- _array_index 1)))) (.location _array_element))) _returnvalue_9) (Math|Conversions|ToFloat(Integer) (Math|Integer|Clamp(Integer) (Math|Float|Floor (/ (Math|Vector|VectorLength (- (.location (Utilities|Array|Get(acopy) (Variables|Default|GetDestination%20Points) (select (select (== _array_index 0) (Variables|Default|GetClose%20Loop?) false) (- (Utilities|Array|Length (Variables|Default|GetDestination%20Points)) 1) (- _array_index 1)))) (.location _array_element))) _returnvalue_9)) 1 (Math|Float|Floor (/ (Math|Vector|VectorLength (- (.location (Utilities|Array|Get(acopy) (Variables|Default|GetDestination%20Points) (select (select (== _array_index 0) (Variables|Default|GetClose%20Loop?) false) (- (Utilities|Array|Length (Variables|Default|GetDestination%20Points)) 1) (- _array_index 1)))) (.location _array_element))) _returnvalue_9))))) (Math|Conversions|ToFloat(Integer) (Math|Integer|Clamp(Integer) (Math|Float|Floor (/ (Math|Vector|VectorLength (- (.location (Utilities|Array|Get(acopy) (Variables|Default|GetDestination%20Points) (select (select (== _array_index 0) (Variables|Default|GetClose%20Loop?) false) (- (Utilities|Array|Length (Variables|Default|GetDestination%20Points)) 1) (- _array_index 1)))) (.location _array_element))) _returnvalue_9)) 1 (Math|Float|Floor (/ (Math|Vector|VectorLength (- (.location (Utilities|Array|Get(acopy) (Variables|Default|GetDestination%20Points) (select (select (== _array_index 0) (Variables|Default|GetClose%20Loop?) false) (- (Utilities|Array|Length (Variables|Default|GetDestination%20Points)) 1) (- _array_index 1)))) (.location _array_element))) _returnvalue_9))))) _returnvalue_9) 0.0))) 0.0 0.0) false true)
                  (if (Variables|Material|GetUse%20Debug%20Material?)
                    (Rendering|Material|SetMaterial _returnvalue_12 0 (Variables|Variables|GetConnecting%20Asset%20Material))
                    (else
                      (Utilities|IsValid _custom_connecting_asset_material_2
                        (:Is%20Valid
                          (Rendering|Material|SetMaterial _returnvalue_12 (Variables|Material|GetCustom%20Connecting%20Asset%20Material%20ID) _custom_connecting_asset_material_2))))))))
            (:then_1
              (bind _returnvalue_13 (AddComponent|AddStaticMeshComponent false (Math|Transform|MakeTransform (.location (Utilities|Array|Get(acopy) (Variables|Default|GetDestination%20Points) (select (select (== _array_index 0) (Variables|Default|GetClose%20Loop?) false) (- (Utilities|Array|Length (Variables|Default|GetDestination%20Points)) 1) (- _array_index 1)))) (Math|Rotator|FindLookatRotation (.location (Utilities|Array|Get(acopy) (Variables|Default|GetDestination%20Points) (select (select (== _array_index 0) (Variables|Default|GetClose%20Loop?) false) (- (Utilities|Array|Length (Variables|Default|GetDestination%20Points)) 1) (- _array_index 1)))) (.location (Utilities|Array|Get(acopy) (Variables|Default|GetDestination%20Points) _array_index))) (Math|Vector|MakeVector (* (select (Variables|Default|GetScale%20assets%20to%20reach%20destination?) (+ 1.0 (/ (- (/ (Math|Vector|VectorLength (- (.location (Utilities|Array|Get(acopy) (Variables|Default|GetDestination%20Points) (select (select (== _array_index 0) (Variables|Default|GetClose%20Loop?) false) (- (Utilities|Array|Length (Variables|Default|GetDestination%20Points)) 1) (- _array_index 1)))) (.location _array_element))) _returnvalue_9) (Math|Conversions|ToFloat(Integer) (Math|Integer|Clamp(Integer) (Math|Float|Floor (/ (Math|Vector|VectorLength (- (.location (Utilities|Array|Get(acopy) (Variables|Default|GetDestination%20Points) (select (select (== _array_index 0) (Variables|Default|GetClose%20Loop?) false) (- (Utilities|Array|Length (Variables|Default|GetDestination%20Points)) 1) (- _array_index 1)))) (.location _array_element))) _returnvalue_9)) 1 (Math|Float|Floor (/ (Math|Vector|VectorLength (- (.location (Utilities|Array|Get(acopy) (Variables|Default|GetDestination%20Points) (select (select (== _array_index 0) (Variables|Default|GetClose%20Loop?) false) (- (Utilities|Array|Length (Variables|Default|GetDestination%20Points)) 1) (- _array_index 1)))) (.location _array_element))) _returnvalue_9))))) (Math|Conversions|ToFloat(Integer) (Math|Integer|Clamp(Integer) (Math|Float|Floor (/ (Math|Vector|VectorLength (- (.location (Utilities|Array|Get(acopy) (Variables|Default|GetDestination%20Points) (select (select (== _array_index 0) (Variables|Default|GetClose%20Loop?) false) (- (Utilities|Array|Length (Variables|Default|GetDestination%20Points)) 1) (- _array_index 1)))) (.location _array_element))) _returnvalue_9)) 1 (Math|Float|Floor (/ (Math|Vector|VectorLength (- (.location (Utilities|Array|Get(acopy) (Variables|Default|GetDestination%20Points) (select (select (== _array_index 0) (Variables|Default|GetClose%20Loop?) false) (- (Utilities|Array|Length (Variables|Default|GetDestination%20Points)) 1) (- _array_index 1)))) (.location _array_element))) _returnvalue_9)))))) 1.0) (+ (/ (Variables|Default|GetAdd%20distance%20to%20Asset%20Length) (- (.x (.max _returnvalue_3)) (.x (.min _returnvalue_3)))) 1.0)) (Variables|Default|GetWidth) (Variables|Default|GetHeight)))))
              (Components|StaticMesh|SetStaticMesh _returnvalue_13 (Variables|Default|GetMain%20Asset))
              (Transformation|AddLocalOffset _returnvalue_13 (Math|Vector|MakeVector (+ (* _index _returnvalue_9) (* _index (select (Variables|Default|GetScale%20assets%20to%20reach%20destination?) (* (/ (- (/ (Math|Vector|VectorLength (- (.location (Utilities|Array|Get(acopy) (Variables|Default|GetDestination%20Points) (select (select (== _array_index 0) (Variables|Default|GetClose%20Loop?) false) (- (Utilities|Array|Length (Variables|Default|GetDestination%20Points)) 1) (- _array_index 1)))) (.location _array_element))) _returnvalue_9) (Math|Conversions|ToFloat(Integer) (Math|Integer|Clamp(Integer) (Math|Float|Floor (/ (Math|Vector|VectorLength (- (.location (Utilities|Array|Get(acopy) (Variables|Default|GetDestination%20Points) (select (select (== _array_index 0) (Variables|Default|GetClose%20Loop?) false) (- (Utilities|Array|Length (Variables|Default|GetDestination%20Points)) 1) (- _array_index 1)))) (.location _array_element))) _returnvalue_9)) 1 (Math|Float|Floor (/ (Math|Vector|VectorLength (- (.location (Utilities|Array|Get(acopy) (Variables|Default|GetDestination%20Points) (select (select (== _array_index 0) (Variables|Default|GetClose%20Loop?) false) (- (Utilities|Array|Length (Variables|Default|GetDestination%20Points)) 1) (- _array_index 1)))) (.location _array_element))) _returnvalue_9))))) (Math|Conversions|ToFloat(Integer) (Math|Integer|Clamp(Integer) (Math|Float|Floor (/ (Math|Vector|VectorLength (- (.location (Utilities|Array|Get(acopy) (Variables|Default|GetDestination%20Points) (select (select (== _array_index 0) (Variables|Default|GetClose%20Loop?) false) (- (Utilities|Array|Length (Variables|Default|GetDestination%20Points)) 1) (- _array_index 1)))) (.location _array_element))) _returnvalue_9)) 1 (Math|Float|Floor (/ (Math|Vector|VectorLength (- (.location (Utilities|Array|Get(acopy) (Variables|Default|GetDestination%20Points) (select (select (== _array_index 0) (Variables|Default|GetClose%20Loop?) false) (- (Utilities|Array|Length (Variables|Default|GetDestination%20Points)) 1) (- _array_index 1)))) (.location _array_element))) _returnvalue_9))))) _returnvalue_9) 0.0))) 0.0 0.0) false true)
              (if (Variables|Material|GetUse%20Debug%20Material?)
                (Rendering|Material|SetMaterial _returnvalue_13 0 (Variables|Variables|GetMain%20Asset%20Material))
                (else
                  (Utilities|IsValid _custom_main_asset_material
                    (:Is%20Valid
                      (Rendering|Material|SetMaterial _returnvalue_13 (Variables|Material|GetCustom%20Main%20Asset%20Material%20ID) _custom_main_asset_material)))))))))
      (else
        (goto _label))))
  (Utilities|IsValid (Variables|Default|GetConnecting%20Asset)
    (:Is%20Valid
      (bind _returnvalue_14 (AddComponent|AddStaticMeshComponent false (Math|Transform|MakeTransform (.location _output) (Math|Rotator|FindLookatRotation (.location _output) (.location (Utilities|Array|Get(acopy) (Variables|Default|GetDestination%20Points) (- _returnvalue_2 2)))) (Math|Vector|MakeVector 1.0 1.0 (Variables|Default|GetHeight)))))
      (Components|StaticMesh|SetStaticMesh _returnvalue_14 (Variables|Default|GetConnecting%20Asset))
      (Transformation|AddLocalOffset _returnvalue_14 (Math|Vector|MakeVector 0.0 0.0 0.0) false true)
      (if (Variables|Material|GetUse%20Debug%20Material?)
        (Rendering|Material|SetMaterial _returnvalue_14 0 (Variables|Variables|GetConnecting%20Asset%20Material))
        (else
          (Utilities|IsValid _custom_connecting_asset_material
            (:Is%20Valid
              (Rendering|Material|SetMaterial _returnvalue_14 (Variables|Material|GetCustom%20Connecting%20Asset%20Material%20ID) _custom_connecting_asset_material))))))))
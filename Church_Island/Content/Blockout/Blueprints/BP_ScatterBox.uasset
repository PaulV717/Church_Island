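; Blockout scatter box that places random static meshes on surrounding surfaces from its construction script.
; Seeded streams drive visibility line traces, cast either along the box's local down axis or inward from random directions toward its center.
; Each hit adds a mesh component with random mesh, scale and rotation, blended toward the surface normal by an alignment strength.
; Optional arrow components preview the trace direction.
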(event EventBeginPlay)

(event Collision|EventActorBeginOverlap
  (params (OtherActor :type Actor%20Object%20Reference)))

(event EventTick
  (params (DeltaSeconds :type Float%20%28single-precision%29)))

(fn ConstructionScript
  (bind _returnvalue (Transformation|GetActorTransform))
  (bind _scale___min (Variables|Default|GetScale%20-%20Min))
  (bind _meshes_to_spawn (Variables|Default|GetMeshes%20To%20Spawn))
  (bind _line_trace_to_center_ (Variables|Default|GetLine%20Trace%20to%20center?))
  (bind _location_seed (Variables|Default|GetLocation%20Seed))
  (bind _location_seed_2 (Variables|Default|GetLocation%20Seed))
  (bind _scale___max (Variables|Default|GetScale%20-%20Max))
  (bind _rotation (Variables|Default|GetRotation))
  (bind _returnvalue_2 (Math|Random|RandomFloatinRangefromStream -1e+03 1e+03 _location_seed))
  (bind _returnvalue_3 (Math|Random|RandomFloatinRangefromStream -1e+03 1e+03 _location_seed))
  (bind _returnvalue_4 (Math|Vector|MakeVector _returnvalue_2 _returnvalue_3 0.0))
  (Transformation|SetRelativeTransform (Variables|Default|GetBox) (Math|Transform|MakeTransform "0, 0, 0" "0, 0, 0" "1,1,1") false false)
  (if (Variables|Default|GetShow%20Linetrace%20Direction?)
    (if (Variables|Default|GetLine%20Trace%20to%20center?)
      (Utilities|FlowControl|Sequence
        (:then_0
          (bind _returnvalue_5 (AddComponent|AddArrowComponent false (Math|Transform|MakeTransform "1500.000000,0.000000,0.000000" "180.000000,0.000000,0.000000" "1,1,1"))) ; Backward
          (Transformation|SetWorldScale3D _returnvalue_5 (Math|Vector|MakeVector (* (.x (Transformation|GetActorScale3D)) 1e+01) 5.0 5.0)))
        (:then_1
          (bind _returnvalue_6 (AddComponent|AddArrowComponent false (Math|Transform|MakeTransform "-1500.000000,0.000000,0.000000" "0.000000,0.000000,0.000000" "1,1,1"))) ; Forward
          (Transformation|SetWorldScale3D _returnvalue_6 (Math|Vector|MakeVector (* (.x (Transformation|GetActorScale3D)) 1e+01) 5.0 5.0)))
        (:then_2
          (bind _returnvalue_7 (AddComponent|AddArrowComponent false (Math|Transform|MakeTransform "0.000000,1500.000000,0.000000" "0.000000,-90.000000,0.000000" "1,1,1"))) ; Right
          (Transformation|SetWorldScale3D _returnvalue_7 (Math|Vector|MakeVector (* (.y (Transformation|GetActorScale3D)) 1e+01) 5.0 5.0)))
        (:then_3
          (bind _returnvalue_8 (AddComponent|AddArrowComponent false (Math|Transform|MakeTransform "0.000000,-1500.000000,0.000000" "0.000000,90.000000,0.000000" "1,1,1"))) ; Left
          (Transformation|SetWorldScale3D _returnvalue_8 (Math|Vector|MakeVector (* (.y (Transformation|GetActorScale3D)) 1e+01) 5.0 5.0)))
        (:then_4
          (bind _returnvalue_9 (AddComponent|AddArrowComponent false (Math|Transform|MakeTransform "0.000000,0.000000,-1500.000000" "90.000000, 0, 0" "1,1,1"))) ; Up
          (Transformation|SetWorldScale3D _returnvalue_9 (Math|Vector|MakeVector (* (.z (Transformation|GetActorScale3D)) 1e+01) 5.0 5.0)))
        (:then_5
          (bind _returnvalue_10 (AddComponent|AddArrowComponent false (Math|Transform|MakeTransform "0.000000,0.000000,1500.000000" "-90.000000, 0, 0" "1,1,1") :!label _label)) ; Down
          (Transformation|SetWorldScale3D _returnvalue_10 (Math|Vector|MakeVector (* (.z (Transformation|GetActorScale3D)) 1e+01) 5.0 5.0))
          (bind _output_get (Variables|Default|SetNumber%20Of%20Meshes (Math|Integer|Clamp(Integer) (Variables|Default|GetNumber%20Of%20Meshes) 1 100) :!label _label_2))
          (for _index (range 1 _output_get)
            (bind (_outhit _returnvalue_11) (Collision|LineTraceByChannel (select _line_trace_to_center_ (Math|Transform|TransformLocation (Transformation|GetActorTransform) (Math|Transform|TransformLocation (Math|Transform|MakeTransform "0, 0, 0" (Math|Rotator|MakeRotator (Math|Random|RandomFloatinRangefromStream -3.6e+02 3.6e+02 _location_seed_2) (Math|Random|RandomFloatinRangefromStream -3.6e+02 3.6e+02 _location_seed_2) (Math|Random|RandomFloatinRangefromStream -3.6e+02 3.6e+02 _location_seed_2)) "1,1,1") "0,0.000000,1000.000000")) (Math|Transform|TransformLocation _returnvalue (+ _returnvalue_4 "0, 0,1000.000000"))) (select _line_trace_to_center_ (Transformation|GetActorLocation) (Math|Transform|TransformLocation _returnvalue (- _returnvalue_4 "0, 0,1000.000000"))) "TraceTypeQuery1" true 0 "None"))
            (if _returnvalue_11
              (bind _returnvalue_12 (AddComponent|AddStaticMeshComponent true (Math|Transform|MakeTransform (.ImpactPoint (Collision|BreakHitResult _outhit)) (Math|Rotator|Lerp(Rotator) (Math|Rotator|MakeRotator 0.0 0.0 (.Yaw (Math|Rotator|BreakRotator (Math|Rotator|MakeRotfromZ (.Normal (Collision|BreakHitResult _outhit)))))) (Math|Rotator|MakeRotfromZ (.Normal (Collision|BreakHitResult _outhit))) (/ (Variables|Default|GetAlign%20To%20Surface%20Strength) 1e+02) true) (Math|Vector|MakeVector (Math|Random|RandomFloatinRangefromStream (.x _scale___min) (.x _scale___max) (Variables|Default|GetScale%20Seed)) (Math|Random|RandomFloatinRangefromStream (.y _scale___min) (.y _scale___max) (Variables|Default|GetScale%20Seed)) (Math|Random|RandomFloatinRangefromStream (.z _scale___min) (.z _scale___max) (Variables|Default|GetScale%20Seed))))))
              (Transformation|SetMobility _returnvalue_12 (Variables|Default|GetSpawned%20Mesh%20Mobility))
              (Transformation|AddLocalRotation _returnvalue_12 (Math|Rotator|MakeRotator (Math|Random|RandomFloatinRangefromStream (* (.roll _rotation) -1.0) (.roll _rotation) (Variables|Default|GetRotation%20Seed)) (Math|Random|RandomFloatinRangefromStream (* (.pitch _rotation) -1.0) (.pitch _rotation) (Variables|Default|GetRotation%20Seed)) (Math|Random|RandomFloatinRangefromStream (* (.yaw _rotation) -1.0) (.yaw _rotation) (Variables|Default|GetRotation%20Seed))) false false)
              (Components|StaticMesh|SetStaticMesh _returnvalue_12 (Utilities|Array|Get(acopy) _meshes_to_spawn (Math|Random|RandomIntegerinRangefromStream 0 (Utilities|Array|LastIndex _meshes_to_spawn) (Variables|Default|GetLocation%20Seed))))))))
      (else
        (goto _label)))
    (else
      (goto _label_2))))
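; Blockout utility pole line that builds poles and sagging powerlines along an editable spline in the construction script.
; Poles are placed by spacing or count, with seeded random mesh, scale and rotation, and take a custom or tinted debug material.
; Up to six spline mesh cables link attachment points on neighbouring poles, using randomised tangent offsets for sag.
; A closed loop adds a final span back to the first pole.
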(event EventBeginPlay)

(event Collision|EventActorBeginOverlap
  (params (OtherActor :type Actor%20Object%20Reference)))

(event EventTick
  (params (DeltaSeconds :type Float%20%28single-precision%29)))

(fn ConstructionScript
  (bind _spline (Variables|Default|GetSpline))
  (bind _scale___min (Variables|Default|GetScale%20-%20Min))
  (bind _pole_meshes_to_spawn (Variables|Default|GetPole%20Meshes%20To%20Spawn))
  (bind _rotate (Variables|Default|GetRotate))
  (bind _scale___max (Variables|Default|GetScale%20-%20Max))
  (bind _spawned_utility_pole_reference (Variables|Reference|GetSpawned%20Utility%20Pole%20Reference))
  (bind _powerline_sag_seed (Variables|Default|GetPowerline%20Sag%20Seed))
  (bind _custom_material (Variables|Material|GetCustom%20Material))
  (bind _count_per_spline (Variables|Default|GetCount%20per%20spline))
  (bind _powerline_sag_strength___max (Variables|Default|GetPowerline%20Sag%20Strength%20-%20Max))
  (bind _spawned_utility_pole_reference_2 (Variables|Reference|GetSpawned%20Utility%20Pole%20Reference))
  (bind _powerline_sag_strength___max_2 (Variables|Default|GetPowerline%20Sag%20Strength%20-%20Max))
  (bind _powerline_sag_seed_2 (Variables|Default|GetPowerline%20Sag%20Seed))
  (bind _spawned_utility_pole_reference_3 (Variables|Reference|GetSpawned%20Utility%20Pole%20Reference))
  (bind _powerline_sag_strength___max_3 (Variables|Default|GetPowerline%20Sag%20Strength%20-%20Max))
  (bind _powerline_sag_seed_3 (Variables|Default|GetPowerline%20Sag%20Seed))
  (bind _powerline_size (Variables|Default|GetPowerline%20Size))
  (bind _powerline_size_2 (Variables|Default|GetPowerline%20Size))
  (bind _powerline_size_3 (Variables|Default|GetPowerline%20Size))
  (bind _powerline_sag_strength___min (Variables|Default|GetPowerline%20Sag%20Strength%20-%20Min))
  (bind _powerline_sag_strength___min_2 (Variables|Default|GetPowerline%20Sag%20Strength%20-%20Min))
  (bind _powerline_sag_strength___min_3 (Variables|Default|GetPowerline%20Sag%20Strength%20-%20Min))
  (bind _spawned_utility_pole_reference_4 (Variables|Reference|GetSpawned%20Utility%20Pole%20Reference))
  (bind _powerline_sag_strength___max_4 (Variables|Default|GetPowerline%20Sag%20Strength%20-%20Max))
  (bind _powerline_sag_seed_4 (Variables|Default|GetPowerline%20Sag%20Seed))
  (bind _powerline_size_4 (Variables|Default|GetPowerline%20Size))
  (bind _powerline_sag_strength___min_4 (Variables|Default|GetPowerline%20Sag%20Strength%20-%20Min))
  (bind _spawned_utility_pole_reference_5 (Variables|Reference|GetSpawned%20Utility%20Pole%20Reference))
  (bind _powerline_sag_strength___max_5 (Variables|Default|GetPowerline%20Sag%20Strength%20-%20Max))
  (bind _powerline_sag_seed_5 (Variables|Default|GetPowerline%20Sag%20Seed))
  (bind _powerline_size_5 (Variables|Default|GetPowerline%20Size))
  (bind _powerline_sag_strength___min_5 (Variables|Default|GetPowerline%20Sag%20Strength%20-%20Min))
  (bind _spawned_utility_pole_reference_6 (Variables|Reference|GetSpawned%20Utility%20Pole%20Reference))
  (bind _powerline_sag_strength___max_6 (Variables|Default|GetPowerline%20Sag%20Strength%20-%20Max))
  (bind _powerline_sag_seed_6 (Variables|Default|GetPowerline%20Sag%20Seed))
  (bind _powerline_size_6 (Variables|Default|GetPowerline%20Size))
  (bind _powerline_sag_strength___min_6 (Variables|Default|GetPowerline%20Sag%20Strength%20-%20Min))
  (bind _returnvalue (Math|Random|RandomFloatinRangefromStream _powerline_sag_strength___min_4 _powerline_sag_strength___max_4 _powerline_sag_seed_4))
  (bind _returnvalue_2 (Math|Random|RandomFloatinRangefromStream _powerline_sag_strength___min_5 _powerline_sag_strength___max_5 _powerline_sag_seed_5))
  (bind _returnvalue_3 (Math|Random|RandomFloatinRangefromStream _powerline_sag_strength___min_6 _powerline_sag_strength___max_6 _powerline_sag_seed_6))
  (bind _returnvalue_4 (Math|Random|RandomFloatinRangefromStream _powerline_sag_strength___min_2 _powerline_sag_strength___max_2 _powerline_sag_seed_2))
  (bind _returnvalue_5 (Math|Random|RandomFloatinRangefromStream _powerline_sag_strength___min_3 _powerline_sag_strength___max_3 _powerline_sag_seed_3))
  (bind _returnvalue_6 (Math|Random|RandomFloatinRangefromStream _powerline_sag_strength___min _powerline_sag_strength___max _powerline_sag_seed))
  (Utilities|Array|Clear (Variables|Reference|GetSpawned%20Utility%20Pole%20Reference))
  (Spline|SetClosedLoop (Variables|Default|GetSpline) (Variables|Default|GetIs%20Closed%20loop?) true)
  (Variables|Variables|SetSpline%20Length (Spline|GetSplineLength (Variables|Default|GetSpline)))
  (Utilities|IsValid (Variables|Material|GetCustom%20Material)
    (:Is%20Valid
      _)
    (:Is%20Not%20Valid
      (if (Variables|Material|GetUse%20Debug%20Material?)
        (bind _returnvalue_7 (Rendering|Material|CreateDynamicMaterialInstance "/Game/Blockout/Material/Base/M_WorldProject.M_WorldProject" "None" :!class /Script/Engine.KismetMaterialLibrary))
        (bind _output_get (Variables|Variables|SetDynamic%20Material _returnvalue_7))
        (Rendering|Material|SetVectorParameterValue _output_get "Diffuse Colour" (Variables|Material|GetSurface%20Colour) :!class /Script/Engine.MaterialInstanceDynamic)
        (Rendering|Material|SetScalarParameterValue _output_get "Unique colour for top?" (Math|Conversions|ToFloat(Boolean) (Variables|Material|GetUnique%20colour%20for%20top?)) :!class /Script/Engine.MaterialInstanceDynamic)
        (Rendering|Material|SetVectorParameterValue _output_get "Diffuse Colour - Top" (Variables|Material|GetTop%20Colour) :!class /Script/Engine.MaterialInstanceDynamic)
        (Rendering|Material|SetScalarParameterValue _output_get "Roughness" (Variables|Material|GetMaterial%20Roughness%20Value) :!class /Script/Engine.MaterialInstanceDynamic))))
  (for _index (range 0 (select (Variables|Default|GetT-Spacing%20F-Count%20per%20spline) (Math|Float|Floor (/ (Variables|Variables|GetSpline%20Length) (Variables|Default|GetSpacing))) (- (Variables|Default|GetCount%20per%20spline) 1)))
    (bind _returnvalue_8 (AddComponent|AddStaticMeshComponent false (Math|Transform|MakeTransform (Spline|GetLocationatDistanceAlongSpline _spline (* _index (select (Variables|Default|GetT-Spacing%20F-Count%20per%20spline) (Variables|Default|GetSpacing) (/ (Variables|Variables|GetSpline%20Length) (Math|Conversions|ToFloat(Integer) (select (Variables|Default|GetIs%20Closed%20loop?) (- _count_per_spline 0) (- _count_per_spline 1)))))) "Local") (select (Variables|Default|GetAlign%20to%20splines%20orientation?) (Math|Conversions|RotationFromXVector (Spline|GetTangentatDistanceAlongSpline _spline (* _index (select (Variables|Default|GetT-Spacing%20F-Count%20per%20spline) (Variables|Default|GetSpacing) (/ (Variables|Variables|GetSpline%20Length) (Math|Conversions|ToFloat(Integer) (select (Variables|Default|GetIs%20Closed%20loop?) (- _count_per_spline 0) (- _count_per_spline 1)))))) "Local")) (Math|Rotator|MakeRotator 0.0 0.0 (.Yaw (Math|Rotator|BreakRotator (Math|Conversions|RotationFromXVector (Spline|GetTangentatDistanceAlongSpline _spline (* _index (select (Variables|Default|GetT-Spacing%20F-Count%20per%20spline) (Variables|Default|GetSpacing) (/ (Variables|Variables|GetSpline%20Length) (Math|Conversions|ToFloat(Integer) (select (Variables|Default|GetIs%20Closed%20loop?) (- _count_per_spline 0) (- _count_per_spline 1)))))) "Local")))))) (Math|Vector|MakeVector (Math|Random|RandomFloatinRangefromStream (.x _scale___min) (.x _scale___max) (Variables|Default|GetScale%20Variation%20Seed)) (Math|Random|RandomFloatinRangefromStream (.y _scale___min) (.y _scale___max) (Variables|Default|GetScale%20Variation%20Seed)) (Math|Random|RandomFloatinRangefromStream (.z _scale___min) (.z _scale___max) (Variables|Default|GetScale%20Variation%20Seed))))))
    (Utilities|Array|Add (Variables|Reference|GetSpawned%20Utility%20Pole%20Reference) _returnvalue_8)
    (Components|StaticMesh|SetStaticMesh _returnvalue_8 (Utilities|Array|Get(acopy) _pole_meshes_to_spawn (Math|Random|RandomIntegerinRangefromStream 0 (Utilities|Array|LastIndex _pole_meshes_to_spawn) (Variables|Default|GetPole%20Variation%20Seed))))
    (Transformation|AddLocalRotation _returnvalue_8 (Math|Rotator|MakeRotator (Math|Random|RandomFloatinRangefromStream (* (.roll _rotate) -1.0) (.roll _rotate) (Variables|Default|GetRotation%20Variation%20Seed)) (Math|Random|RandomFloatinRangefromStream (* (.pitch _rotate) -1.0) (.pitch _rotate) (Variables|Default|GetRotation%20Variation%20Seed)) (Math|Random|RandomFloatinRangefromStream (* (.yaw _rotate) -1.0) (.yaw _rotate) (Variables|Default|GetRotation%20Variation%20Seed))) false false)
    (Utilities|IsValid _custom_material
      (:Is%20Valid
        (Rendering|Material|SetMaterial _returnvalue_8 (Variables|Material|GetCustom%20Material%20ID) _custom_material)
        (if (not (== _index 0)) :!label _label
          (Utilities|FlowControl|Sequence
            (:then_0
              (if (Variables|Default|GetUse%20Powerline%201?)
                (bind _returnvalue_9 (AddComponent|AddSplineMeshComponent false))
                (Components|StaticMesh|SetStaticMesh _returnvalue_9 (Variables|Default|GetNew%20Cable%20Mesh))
                (SplineMesh|SetStartandEnd _returnvalue_9 (Math|Transform|TransformLocation (Transformation|GetRelativeTransform (Utilities|Array|Get(acopy) _spawned_utility_pole_reference_2 (- _index 1))) (.location (Variables|PowerlineLocation|GetPowerline%201A))) (- (* (Math|Rotator|GetRotationXVector (Math|Rotator|FindLookatRotation (Math|Transform|TransformLocation (Transformation|GetRelativeTransform (Utilities|Array|Get(acopy) _spawned_utility_pole_reference_2 (- _index 1))) (.location (Variables|PowerlineLocation|GetPowerline%201A))) (Math|Transform|TransformLocation (Transformation|GetRelativeTransform (Utilities|Array|Get(acopy) _spawned_utility_pole_reference_2 (select (== _index (Variables|Default|GetCount%20per%20spline)) 0 _index))) (.location (Variables|PowerlineLocation|GetPowerline%201B))))) (Math|Vector|VectorLength (- (Math|Transform|TransformLocation (Transformation|GetRelativeTransform (Utilities|Array|Get(acopy) _spawned_utility_pole_reference_2 (- _index 1))) (.location (Variables|PowerlineLocation|GetPowerline%201A))) (Math|Transform|TransformLocation (Transformation|GetRelativeTransform (Utilities|Array|Get(acopy) _spawned_utility_pole_reference_2 (select (== _index (Variables|Default|GetCount%20per%20spline)) 0 _index))) (.location (Variables|PowerlineLocation|GetPowerline%201B)))))) (Math|Vector|MakeVector 0.0 0.0 _returnvalue_4)) (Math|Transform|TransformLocation (Transformation|GetRelativeTransform (Utilities|Array|Get(acopy) _spawned_utility_pole_reference_2 (select (== _index (Variables|Default|GetCount%20per%20spline)) 0 _index))) (.location (Variables|PowerlineLocation|GetPowerline%201B))) (+ (* (Math|Rotator|GetRotationXVector (Math|Rotator|FindLookatRotation (Math|Transform|TransformLocation (Transformation|GetRelativeTransform (Utilities|Array|Get(acopy) _spawned_utility_pole_reference_2 (- _index 1))) (.location (Variables|PowerlineLocation|GetPowerline%201A))) (Math|Transform|TransformLocation (Transformation|GetRelativeTransform (Utilities|Array|Get(acopy) _spawned_utility_pole_reference_2 (select (== _index (Variables|Default|GetCount%20per%20spline)) 0 _index))) (.location (Variables|PowerlineLocation|GetPowerline%201B))))) (Math|Vector|VectorLength (- (Math|Transform|TransformLocation (Transformation|GetRelativeTransform (Utilities|Array|Get(acopy) _spawned_utility_pole_reference_2 (- _index 1))) (.location (Variables|PowerlineLocation|GetPowerline%201A))) (Math|Transform|TransformLocation (Transformation|GetRelativeTransform (Utilities|Array|Get(acopy) _spawned_utility_pole_reference_2 (select (== _index (Variables|Default|GetCount%20per%20spline)) 0 _index))) (.location (Variables|PowerlineLocation|GetPowerline%201B)))))) (Math|Vector|MakeVector 0.0 0.0 _returnvalue_4)) true :!class /Script/Engine.SplineMeshComponent)
                (SplineMesh|SetStartScale _returnvalue_9 (Math|Vector2D|MakeVector2D _powerline_size_3 _powerline_size_3) true :!class /Script/Engine.SplineMeshComponent)
                (SplineMesh|SetEndScale _returnvalue_9 (Math|Vector2D|MakeVector2D _powerline_size_3 _powerline_size_3) true :!class /Script/Engine.SplineMeshComponent)))
            (:then_1
              (if (Variables|Default|GetUse%20Powerline%202?)
                (bind _returnvalue_10 (AddComponent|AddSplineMeshComponent false))
                (Components|StaticMesh|SetStaticMesh _returnvalue_10 (Variables|Default|GetNew%20Cable%20Mesh))
                (SplineMesh|SetStartandEnd _returnvalue_10 (Math|Transform|TransformLocation (Transformation|GetRelativeTransform (Utilities|Array|Get(acopy) _spawned_utility_pole_reference_3 (- _index 1))) (.location (Variables|PowerlineLocation|GetPowerline%202A))) (- (* (Math|Rotator|GetRotationXVector (Math|Rotator|FindLookatRotation (Math|Transform|TransformLocation (Transformation|GetRelativeTransform (Utilities|Array|Get(acopy) _spawned_utility_pole_reference_3 (- _index 1))) (.location (Variables|PowerlineLocation|GetPowerline%202A))) (Math|Transform|TransformLocation (Transformation|GetRelativeTransform (Utilities|Array|Get(acopy) _spawned_utility_pole_reference_3 (select (== _index (Variables|Default|GetCount%20per%20spline)) 0 _index))) (.location (Variables|PowerlineLocation|GetPowerline%202B))))) (Math|Vector|VectorLength (- (Math|Transform|TransformLocation (Transformation|GetRelativeTransform (Utilities|Array|Get(acopy) _spawned_utility_pole_reference_3 (- _index 1))) (.location (Variables|PowerlineLocation|GetPowerline%202A))) (Math|Transform|TransformLocation (Transformation|GetRelativeTransform (Utilities|Array|Get(acopy) _spawned_utility_pole_reference_3 (select (== _index (Variables|Default|GetCount%20per%20spline)) 0 _index))) (.location (Variables|PowerlineLocation|GetPowerline%202B)))))) (Math|Vector|MakeVector 0.0 0.0 _returnvalue_5)) (Math|Transform|TransformLocation (Transformation|GetRelativeTransform (Utilities|Array|Get(acopy) _spawned_utility_pole_reference_3 (select (== _index (Variables|Default|GetCount%20per%20spline)) 0 _index))) (.location (Variables|PowerlineLocation|GetPowerline%202B))) (+ (* (Math|Rotator|GetRotationXVector (Math|Rotator|FindLookatRotation (Math|Transform|TransformLocation (Transformation|GetRelativeTransform (Utilities|Array|Get(acopy) _spawned_utility_pole_reference_3 (- _index 1))) (.location (Variables|PowerlineLocation|GetPowerline%202A))) (Math|Transform|TransformLocation (Transformation|GetRelativeTransform (Utilities|Array|Get(acopy) _spawned_utility_pole_reference_3 (select (== _index (Variables|Default|GetCount%20per%20spline)) 0 _index))) (.location (Variables|PowerlineLocation|GetPowerline%202B))))) (Math|Vector|VectorLength (- (Math|Transform|TransformLocation (Transformation|GetRelativeTransform (Utilities|Array|Get(acopy) _spawned_utility_pole_reference_3 (- _index 1))) (.location (Variables|PowerlineLocation|GetPowerline%202A))) (Math|Transform|TransformLocation (Transformation|GetRelativeTransform (Utilities|Array|Get(acopy) _spawned_utility_pole_reference_3 (select (== _index (Variables|Default|GetCount%20per%20spline)) 0 _index))) (.location (Variables|PowerlineLocation|GetPowerline%202B)))))) (Math|Vector|MakeVector 0.0 0.0 _returnvalue_5)) true :!class /Script/Engine.SplineMeshComponent)
                (SplineMesh|SetStartScale _returnvalue_10 (Math|Vector2D|MakeVector2D _powerline_size_2 _powerline_size_2) true :!class /Script/Engine.SplineMeshComponent)
                (SplineMesh|SetEndScale _returnvalue_10 (Math|Vector2D|MakeVector2D _powerline_size_2 _powerline_size_2) true :!class /Script/Engine.SplineMeshComponent)))
            (:then_2
              (if (Variables|Default|GetUse%20Powerline%203?)
                (bind _returnvalue_11 (AddComponent|AddSplineMeshComponent false))
                (Components|StaticMesh|SetStaticMesh _returnvalue_11 (Variables|Default|GetNew%20Cable%20Mesh))
                (SplineMesh|SetStartandEnd _returnvalue_11 (Math|Transform|TransformLocation (Transformation|GetRelativeTransform (Utilities|Array|Get(acopy) _spawned_utility_pole_reference_4 (- _index 1))) (.location (Variables|PowerlineLocation|GetPowerline%203A))) (- (* (Math|Rotator|GetRotationXVector (Math|Rotator|FindLookatRotation (Math|Transform|TransformLocation (Transformation|GetRelativeTransform (Utilities|Array|Get(acopy) _spawned_utility_pole_reference_4 (- _index 1))) (.location (Variables|PowerlineLocation|GetPowerline%203A))) (Math|Transform|TransformLocation (Transformation|GetRelativeTransform (Utilities|Array|Get(acopy) _spawned_utility_pole_reference_4 (select (== _index (Variables|Default|GetCount%20per%20spline)) 0 _index))) (.location (Variables|PowerlineLocation|GetPowerline%203B))))) (Math|Vector|VectorLength (- (Math|Transform|TransformLocation (Transformation|GetRelativeTransform (Utilities|Array|Get(acopy) _spawned_utility_pole_reference_4 (- _index 1))) (.location (Variables|PowerlineLocation|GetPowerline%203A))) (Math|Transform|TransformLocation (Transformation|GetRelativeTransform (Utilities|Array|Get(acopy) _spawned_utility_pole_reference_4 (select (== _index (Variables|Default|GetCount%20per%20spline)) 0 _index))) (.location (Variables|PowerlineLocation|GetPowerline%203B)))))) (Math|Vector|MakeVector 0.0 0.0 _returnvalue)) (Math|Transform|TransformLocation (Transformation|GetRelativeTransform (Utilities|Array|Get(acopy) _spawned_utility_pole_reference_4 (select (== _index (Variables|Default|GetCount%20per%20spline)) 0 _index))) (.location (Variables|PowerlineLocation|GetPowerline%203B))) (+ (* (Math|Rotator|GetRotationXVector (Math|Rotator|FindLookatRotation (Math|Transform|TransformLocation (Transformation|GetRelativeTransform (Utilities|Array|Get(acopy) _spawned_utility_pole_reference_4 (- _index 1))) (.location (Variables|PowerlineLocation|GetPowerline%203A))) (Math|Transform|TransformLocation (Transformation|GetRelativeTransform (Utilities|Array|Get(acopy) _spawned_utility_pole_reference_4 (select (== _index (Variables|Default|GetCount%20per%20spline)) 0 _index))) (.location (Variables|PowerlineLocation|GetPowerline%203B))))) (Math|Vector|VectorLength (- (Math|Transform|TransformLocation (Transformation|GetRelativeTransform (Utilities|Array|Get(acopy) _spawned_utility_pole_reference_4 (- _index 1))) (.location (Variables|PowerlineLocation|GetPowerline%203A))) (Math|Transform|TransformLocation (Transformation|GetRelativeTransform (Utilities|Array|Get(acopy) _spawned_utility_pole_reference_4 (select (== _index (Variables|Default|GetCount%20per%20spline)) 0 _index))) (.location (Variables|PowerlineLocation|GetPowerline%203B)))))) (Math|Vector|MakeVector 0.0 0.0 _returnvalue)) true :!class /Script/Engine.SplineMeshComponent)
                (SplineMesh|SetStartScale _returnvalue_11 (Math|Vector2D|MakeVector2D _powerline_size_4 _powerline_size_4) true :!class /Script/Engine.SplineMeshComponent)
                (SplineMesh|SetEndScale _returnvalue_11 (Math|Vector2D|MakeVector2D _powerline_size_4 _powerline_size_4) true :!class /Script/Engine.SplineMeshComponent)))
            (:then_3
              (if (Variables|Default|GetUse%20Powerline%204?)
                (bind _returnvalue_12 (AddComponent|AddSplineMeshComponent false))
                (Components|StaticMesh|SetStaticMesh _returnvalue_12 (Variables|Default|GetNew%20Cable%20Mesh))
                (SplineMesh|SetStartandEnd _returnvalue_12 (Math|Transform|TransformLocation (Transformation|GetRelativeTransform (Utilities|Array|Get(acopy) _spawned_utility_pole_reference_5 (- _index 1))) (.location (Variables|PowerlineLocation|GetPowerline%204A))) (- (* (Math|Rotator|GetRotationXVector (Math|Rotator|FindLookatRotation (Math|Transform|TransformLocation (Transformation|GetRelativeTransform (Utilities|Array|Get(acopy) _spawned_utility_pole_reference_5 (- _index 1))) (.location (Variables|PowerlineLocation|GetPowerline%204A))) (Math|Transform|TransformLocation (Transformation|GetRelativeTransform (Utilities|Array|Get(acopy) _spawned_utility_pole_reference_5 (select (== _index (Variables|Default|GetCount%20per%20spline)) 0 _index))) (.location (Variables|PowerlineLocation|GetPowerline%204B))))) (Math|Vector|VectorLength (- (Math|Transform|TransformLocation (Transformation|GetRelativeTransform (Utilities|Array|Get(acopy) _spawned_utility_pole_reference_5 (- _index 1))) (.location (Variables|PowerlineLocation|GetPowerline%204A))) (Math|Transform|TransformLocation (Transformation|GetRelativeTransform (Utilities|Array|Get(acopy) _spawned_utility_pole_reference_5 (select (== _index (Variables|Default|GetCount%20per%20spline)) 0 _index))) (.location (Variables|PowerlineLocation|GetPowerline%204B)))))) (Math|Vector|MakeVector 0.0 0.0 _returnvalue_2)) (Math|Transform|TransformLocation (Transformation|GetRelativeTransform (Utilities|Array|Get(acopy) _spawned_utility_pole_reference_5 (select (== _index (Variables|Default|GetCount%20per%20spline)) 0 _index))) (.location (Variables|PowerlineLocation|GetPowerline%204B))) (+ (* (Math|Rotator|GetRotationXVector (Math|Rotator|FindLookatRotation (Math|Transform|TransformLocation (Transformation|GetRelativeTransform (Utilities|Array|Get(acopy) _spawned_utility_pole_reference_5 (- _index 1))) (.location (Variables|PowerlineLocation|GetPowerline%204A))) (Math|Transform|TransformLocation (Transformation|GetRelativeTransform (Utilities|Array|Get(acopy) _spawned_utility_pole_reference_5 (select (== _index (Variables|Default|GetCount%20per%20spline)) 0 _index))) (.location (Variables|PowerlineLocation|GetPowerline%204B))))) (Math|Vector|VectorLength (- (Math|Transform|TransformLocation (Transformation|GetRelativeTransform (Utilities|Array|Get(acopy) _spawned_utility_pole_reference_5 (- _index 1))) (.location (Variables|PowerlineLocation|GetPowerline%204A))) (Math|Transform|TransformLocation (Transformation|GetRelativeTransform (Utilities|Array|Get(acopy) _spawned_utility_pole_reference_5 (select (== _index (Variables|Default|GetCount%20per%20spline)) 0 _index))) (.location (Variables|PowerlineLocation|GetPowerline%204B)))))) (Math|Vector|MakeVector 0.0 0.0 _returnvalue_2)) true :!class /Script/Engine.SplineMeshComponent)
                (SplineMesh|SetStartScale _returnvalue_12 (Math|Vector2D|MakeVector2D _powerline_size_5 _powerline_size_5) true :!class /Script/Engine.SplineMeshComponent)
                (SplineMesh|SetEndScale _returnvalue_12 (Math|Vector2D|MakeVector2D _powerline_size_5 _powerline_size_5) true :!class /Script/Engine.SplineMeshComponent)))
            (:then_4
              (if (Variables|Default|GetUse%20Powerline%205?)
                (bind _returnvalue_13 (AddComponent|AddSplineMeshComponent false))
                (Components|StaticMesh|SetStaticMesh _returnvalue_13 (Variables|Default|GetNew%20Cable%20Mesh))
                (SplineMesh|SetStartandEnd _returnvalue_13 (Math|Transform|TransformLocation (Transformation|GetRelativeTransform (Utilities|Array|Get(acopy) _spawned_utility_pole_reference_6 (- _index 1))) (.location (Variables|PowerlineLocation|GetPowerline%205A))) (- (* (Math|Rotator|GetRotationXVector (Math|Rotator|FindLookatRotation (Math|Transform|TransformLocation (Transformation|GetRelativeTransform (Utilities|Array|Get(acopy) _spawned_utility_pole_reference_6 (- _index 1))) (.location (Variables|PowerlineLocation|GetPowerline%205A))) (Math|Transform|TransformLocation (Transformation|GetRelativeTransform (Utilities|Array|Get(acopy) _spawned_utility_pole_reference_6 (select (== _index (Variables|Default|GetCount%20per%20spline)) 0 _index))) (.location (Variables|PowerlineLocation|GetPowerline%205B))))) (Math|Vector|VectorLength (- (Math|Transform|TransformLocation (Transformation|GetRelativeTransform (Utilities|Array|Get(acopy) _spawned_utility_pole_reference_6 (- _index 1))) (.location (Variables|PowerlineLocation|GetPowerline%205A))) (Math|Transform|TransformLocation (Transformation|GetRelativeTransform (Utilities|Array|Get(acopy) _spawned_utility_pole_reference_6 (select (== _index (Variables|Default|GetCount%20per%20spline)) 0 _index))) (.location (Variables|PowerlineLocation|GetPowerline%205B)))))) (Math|Vector|MakeVector 0.0 0.0 _returnvalue_3)) (Math|Transform|TransformLocation (Transformation|GetRelativeTransform (Utilities|Array|Get(acopy) _spawned_utility_pole_reference_6 (select (== _index (Variables|Default|GetCount%20per%20spline)) 0 _index))) (.location (Variables|PowerlineLocation|GetPowerline%205B))) (+ (* (Math|Rotator|GetRotationXVector (Math|Rotator|FindLookatRotation (Math|Transform|TransformLocation (Transformation|GetRelativeTransform (Utilities|Array|Get(acopy) _spawned_utility_pole_reference_6 (- _index 1))) (.location (Variables|PowerlineLocation|GetPowerline%205A))) (Math|Transform|TransformLocation (Transformation|GetRelativeTransform (Utilities|Array|Get(acopy) _spawned_utility_pole_reference_6 (select (== _index (Variables|Default|GetCount%20per%20spline)) 0 _index))) (.location (Variables|PowerlineLocation|GetPowerline%205B))))) (Math|Vector|VectorLength (- (Math|Transform|TransformLocation (Transformation|GetRelativeTransform (Utilities|Array|Get(acopy) _spawned_utility_pole_reference_6 (- _index 1))) (.location (Variables|PowerlineLocation|GetPowerline%205A))) (Math|Transform|TransformLocation (Transformation|GetRelativeTransform (Utilities|Array|Get(acopy) _spawned_utility_pole_reference_6 (select (== _index (Variables|Default|GetCount%20per%20spline)) 0 _index))) (.location (Variables|PowerlineLocation|GetPowerline%205B)))))) (Math|Vector|MakeVector 0.0 0.0 _returnvalue_3)) true :!class /Script/Engine.SplineMeshComponent)
                (SplineMesh|SetStartScale _returnvalue_13 (Math|Vector2D|MakeVector2D _powerline_size_6 _powerline_size_6) true :!class /Script/Engine.SplineMeshComponent)
                (SplineMesh|SetEndScale _returnvalue_13 (Math|Vector2D|MakeVector2D _powerline_size_6 _powerline_size_6) true :!class /Script/Engine.SplineMeshComponent)))
            (:then_5
              (if (Variables|Default|GetUse%20Powerline%206?)
                (bind _returnvalue_14 (AddComponent|AddSplineMeshComponent false))
                (Components|StaticMesh|SetStaticMesh _returnvalue_14 (Variables|Default|GetNew%20Cable%20Mesh))
                (SplineMesh|SetStartandEnd _returnvalue_14 (Math|Transform|TransformLocation (Transformation|GetRelativeTransform (Utilities|Array|Get(acopy) _spawned_utility_pole_reference (- _index 1))) (.location (Variables|PowerlineLocation|GetPowerline%206A))) (- (* (Math|Rotator|GetRotationXVector (Math|Rotator|FindLookatRotation (Math|Transform|TransformLocation (Transformation|GetRelativeTransform (Utilities|Array|Get(acopy) _spawned_utility_pole_reference (- _index 1))) (.location (Variables|PowerlineLocation|GetPowerline%206A))) (Math|Transform|TransformLocation (Transformation|GetRelativeTransform (Utilities|Array|Get(acopy) _spawned_utility_pole_reference (select (== _index (Variables|Default|GetCount%20per%20spline)) 0 _index))) (.location (Variables|PowerlineLocation|GetPowerline%206B))))) (Math|Vector|VectorLength (- (Math|Transform|TransformLocation (Transformation|GetRelativeTransform (Utilities|Array|Get(acopy) _spawned_utility_pole_reference (- _index 1))) (.location (Variables|PowerlineLocation|GetPowerline%206A))) (Math|Transform|TransformLocation (Transformation|GetRelativeTransform (Utilities|Array|Get(acopy) _spawned_utility_pole_reference (select (== _index (Variables|Default|GetCount%20per%20spline)) 0 _index))) (.location (Variables|PowerlineLocation|GetPowerline%206B)))))) (Math|Vector|MakeVector 0.0 0.0 _returnvalue_6)) (Math|Transform|TransformLocation (Transformation|GetRelativeTransform (Utilities|Array|Get(acopy) _spawned_utility_pole_reference (select (== _index (Variables|Default|GetCount%20per%20spline)) 0 _index))) (.location (Variables|PowerlineLocation|GetPowerline%206B))) (+ (* (Math|Rotator|GetRotationXVector (Math|Rotator|FindLookatRotation (Math|Transform|TransformLocation (Transformation|GetRelativeTransform (Utilities|Array|Get(acopy) _spawned_utility_pole_reference (- _index 1))) (.location (Variables|PowerlineLocation|GetPowerline%206A))) (Math|Transform|TransformLocation (Transformation|GetRelativeTransform (Utilities|Array|Get(acopy) _spawned_utility_pole_reference (select (== _index (Variables|Default|GetCount%20per%20spline)) 0 _index))) (.location (Variables|PowerlineLocation|GetPowerline%206B))))) (Math|Vector|VectorLength (- (Math|Transform|TransformLocation (Transformation|GetRelativeTransform (Utilities|Array|Get(acopy) _spawned_utility_pole_reference (- _index 1))) (.location (Variables|PowerlineLocation|GetPowerline%206A))) (Math|Transform|TransformLocation (Transformation|GetRelativeTransform (Utilities|Array|Get(acopy) _spawned_utility_pole_reference (select (== _index (Variables|Default|GetCount%20per%20spline)) 0 _index))) (.location (Variables|PowerlineLocation|GetPowerline%206B)))))) (Math|Vector|MakeVector 0.0 0.0 _returnvalue_6)) true :!class /Script/Engine.SplineMeshComponent)
                (SplineMesh|SetStartScale _returnvalue_14 (Math|Vector2D|MakeVector2D _powerline_size _powerline_size) true :!class /Script/Engine.SplineMeshComponent)
                (SplineMesh|SetEndScale _returnvalue_14 (Math|Vector2D|MakeVector2D _powerline_size _powerline_size) true :!class /Script/Engine.SplineMeshComponent))))))
      (:Is%20Not%20Valid
        (if (Variables|Material|GetUse%20Debug%20Material?)
          (Rendering|Material|SetMaterial _returnvalue_8 0 (Variables|Variables|GetDynamic%20Material))
          (goto _label)))))
  (if (Variables|Default|GetIs%20Closed%20loop?)
    (Utilities|FlowControl|Sequence
      (:then_0
        (if (Variables|Default|GetUse%20Powerline%201?)
          (bind _returnvalue_15 (AddComponent|AddSplineMeshComponent false))
          (Components|StaticMesh|SetStaticMesh _returnvalue_15 (Variables|Default|GetNew%20Cable%20Mesh))
          (SplineMesh|SetStartandEnd _returnvalue_15 (Math|Transform|TransformLocation (Transformation|GetRelativeTransform (Utilities|Array|Get(acopy) _spawned_utility_pole_reference_2 (- _index 1))) (.location (Variables|PowerlineLocation|GetPowerline%201A))) (- (* (Math|Rotator|GetRotationXVector (Math|Rotator|FindLookatRotation (Math|Transform|TransformLocation (Transformation|GetRelativeTransform (Utilities|Array|Get(acopy) _spawned_utility_pole_reference_2 (- _index 1))) (.location (Variables|PowerlineLocation|GetPowerline%201A))) (Math|Transform|TransformLocation (Transformation|GetRelativeTransform (Utilities|Array|Get(acopy) _spawned_utility_pole_reference_2 (select (== _index (Variables|Default|GetCount%20per%20spline)) 0 _index))) (.location (Variables|PowerlineLocation|GetPowerline%201B))))) (Math|Vector|VectorLength (- (Math|Transform|TransformLocation (Transformation|GetRelativeTransform (Utilities|Array|Get(acopy) _spawned_utility_pole_reference_2 (- _index 1))) (.location (Variables|PowerlineLocation|GetPowerline%201A))) (Math|Transform|TransformLocation (Transformation|GetRelativeTransform (Utilities|Array|Get(acopy) _spawned_utility_pole_reference_2 (select (== _index (Variables|Default|GetCount%20per%20spline)) 0 _index))) (.location (Variables|PowerlineLocation|GetPowerline%201B)))))) (Math|Vector|MakeVector 0.0 0.0 _returnvalue_4)) (Math|Transform|TransformLocation (Transformation|GetRelativeTransform (Utilities|Array|Get(acopy) _spawned_utility_pole_reference_2 (select (== _index (Variables|Default|GetCount%20per%20spline)) 0 _index))) (.location (Variables|PowerlineLocation|GetPowerline%201B))) (+ (* (Math|Rotator|GetRotationXVector (Math|Rotator|FindLookatRotation (Math|Transform|TransformLocation (Transformation|GetRelativeTransform (Utilities|Array|Get(acopy) _spawned_utility_pole_reference_2 (- _index 1))) (.location (Variables|PowerlineLocation|GetPowerline%201A))) (Math|Transform|TransformLocation (Transformation|GetRelativeTransform (Utilities|Array|Get(acopy) _spawned_utility_pole_reference_2 (select (== _index (Variables|Default|GetCount%20per%20spline)) 0 _index))) (.location (Variables|PowerlineLocation|GetPowerline%201B))))) (Math|Vector|VectorLength (- (Math|Transform|TransformLocation (Transformation|GetRelativeTransform (Utilities|Array|Get(acopy) _spawned_utility_pole_reference_2 (- _index 1))) (.location (Variables|PowerlineLocation|GetPowerline%201A))) (Math|Transform|TransformLocation (Transformation|GetRelativeTransform (Utilities|Array|Get(acopy) _spawned_utility_pole_reference_2 (select (== _index (Variables|Default|GetCount%20per%20spline)) 0 _index))) (.location (Variables|PowerlineLocation|GetPowerline%201B)))))) (Math|Vector|MakeVector 0.0 0.0 _returnvalue_4)) true :!class /Script/Engine.SplineMeshComponent)
          (SplineMesh|SetStartScale _returnvalue_15 (Math|Vector2D|MakeVector2D _powerline_size_3 _powerline_size_3) true :!class /Script/Engine.SplineMeshComponent)
          (SplineMesh|SetEndScale _returnvalue_15 (Math|Vector2D|MakeVector2D _powerline_size_3 _powerline_size_3) true :!class /Script/Engine.SplineMeshComponent)))
      (:then_1
        (if (Variables|Default|GetUse%20Powerline%202?)
          (bind _returnvalue_16 (AddComponent|AddSplineMeshComponent false))
          (Components|StaticMesh|SetStaticMesh _returnvalue_16 (Variables|Default|GetNew%20Cable%20Mesh))
          (SplineMesh|SetStartandEnd _returnvalue_16 (Math|Transform|TransformLocation (Transformation|GetRelativeTransform (Utilities|Array|Get(acopy) _spawned_utility_pole_reference_3 (- _index 1))) (.location (Variables|PowerlineLocation|GetPowerline%202A))) (- (* (Math|Rotator|GetRotationXVector (Math|Rotator|FindLookatRotation (Math|Transform|TransformLocation (Transformation|GetRelativeTransform (Utilities|Array|Get(acopy) _spawned_utility_pole_reference_3 (- _index 1))) (.location (Variables|PowerlineLocation|GetPowerline%202A))) (Math|Transform|TransformLocation (Transformation|GetRelativeTransform (Utilities|Array|Get(acopy) _spawned_utility_pole_reference_3 (select (== _index (Variables|Default|GetCount%20per%20spline)) 0 _index))) (.location (Variables|PowerlineLocation|GetPowerline%202B))))) (Math|Vector|VectorLength (- (Math|Transform|TransformLocation (Transformation|GetRelativeTransform (Utilities|Array|Get(acopy) _spawned_utility_pole_reference_3 (- _index 1))) (.location (Variables|PowerlineLocation|GetPowerline%202A))) (Math|Transform|TransformLocation (Transformation|GetRelativeTransform (Utilities|Array|Get(acopy) _spawned_utility_pole_reference_3 (select (== _index (Variables|Default|GetCount%20per%20spline)) 0 _index))) (.location (Variables|PowerlineLocation|GetPowerline%202B)))))) (Math|Vector|MakeVector 0.0 0.0 _returnvalue_5)) (Math|Transform|TransformLocation (Transformation|GetRelativeTransform (Utilities|Array|Get(acopy) _spawned_utility_pole_reference_3 (select (== _index (Variables|Default|GetCount%20per%20spline)) 0 _index))) (.location (Variables|PowerlineLocation|GetPowerline%202B))) (+ (* (Math|Rotator|GetRotationXVector (Math|Rotator|FindLookatRotation (Math|Transform|TransformLocation (Transformation|GetRelativeTransform (Utilities|Array|Get(acopy) _spawned_utility_pole_reference_3 (- _index 1))) (.location (Variables|PowerlineLocation|GetPowerline%202A))) (Math|Transform|TransformLocation (Transformation|GetRelativeTransform (Utilities|Array|Get(acopy) _spawned_utility_pole_reference_3 (select (== _index (Variables|Default|GetCount%20per%20spline)) 0 _index))) (.location (Variables|PowerlineLocation|GetPowerline%202B))))) (Math|Vector|VectorLength (- (Math|Transform|TransformLocation (Transformation|GetRelativeTransform (Utilities|Array|Get(acopy) _spawned_utility_pole_reference_3 (- _index 1))) (.location (Variables|PowerlineLocation|GetPowerline%202A))) (Math|Transform|TransformLocation (Transformation|GetRelativeTransform (Utilities|Array|Get(acopy) _spawned_utility_pole_reference_3 (select (== _index (Variables|Default|GetCount%20per%20spline)) 0 _index))) (.location (Variables|PowerlineLocation|GetPowerline%202B)))))) (Math|Vector|MakeVector 0.0 0.0 _returnvalue_5)) true :!class /Script/Engine.SplineMeshComponent)
          (SplineMesh|SetStartScale _returnvalue_16 (Math|Vector2D|MakeVector2D _powerline_size_2 _powerline_size_2) true :!class /Script/Engine.SplineMeshComponent)
          (SplineMesh|SetEndScale _returnvalue_16 (Math|Vector2D|MakeVector2D _powerline_size_2 _powerline_size_2) true :!class /Script/Engine.SplineMeshComponent)))
      (:then_2
        (if (Variables|Default|GetUse%20Powerline%203?)
          (bind _returnvalue_17 (AddComponent|AddSplineMeshComponent false))
          (Components|StaticMesh|SetStaticMesh _returnvalue_17 (Variables|Default|GetNew%20Cable%20Mesh))
          (SplineMesh|SetStartandEnd _returnvalue_17 (Math|Transform|TransformLocation (Transformation|GetRelativeTransform (Utilities|Array|Get(acopy) _spawned_utility_pole_reference_4 (- _index 1))) (.location (Variables|PowerlineLocation|GetPowerline%203A))) (- (* (Math|Rotator|GetRotationXVector (Math|Rotator|FindLookatRotation (Math|Transform|TransformLocation (Transformation|GetRelativeTransform (Utilities|Array|Get(acopy) _spawned_utility_pole_reference_4 (- _index 1))) (.location (Variables|PowerlineLocation|GetPowerline%203A))) (Math|Transform|TransformLocation (Transformation|GetRelativeTransform (Utilities|Array|Get(acopy) _spawned_utility_pole_reference_4 (select (== _index (Variables|Default|GetCount%20per%20spline)) 0 _index))) (.location (Variables|PowerlineLocation|GetPowerline%203B))))) (Math|Vector|VectorLength (- (Math|Transform|TransformLocation (Transformation|GetRelativeTransform (Utilities|Array|Get(acopy) _spawned_utility_pole_reference_4 (- _index 1))) (.location (Variables|PowerlineLocation|GetPowerline%203A))) (Math|Transform|TransformLocation (Transformation|GetRelativeTransform (Utilities|Array|Get(acopy) _spawned_utility_pole_reference_4 (select (== _index (Variables|Default|GetCount%20per%20spline)) 0 _index))) (.location (Variables|PowerlineLocation|GetPowerline%203B)))))) (Math|Vector|MakeVector 0.0 0.0 _returnvalue)) (Math|Transform|TransformLocation (Transformation|GetRelativeTransform (Utilities|Array|Get(acopy) _spawned_utility_pole_reference_4 (select (== _index (Variables|Default|GetCount%20per%20spline)) 0 _index))) (.location (Variables|PowerlineLocation|GetPowerline%203B))) (+ (* (Math|Rotator|GetRotationXVector (Math|Rotator|FindLookatRotation (Math|Transform|TransformLocation (Transformation|GetRelativeTransform (Utilities|Array|Get(acopy) _spawned_utility_pole_reference_4 (- _index 1))) (.location (Variables|PowerlineLocation|GetPowerline%203A))) (Math|Transform|TransformLocation (Transformation|GetRelativeTransform (Utilities|Array|Get(acopy) _spawned_utility_pole_reference_4 (select (== _index (Variables|Default|GetCount%20per%20spline)) 0 _index))) (.location (Variables|PowerlineLocation|GetPowerline%203B))))) (Math|Vector|VectorLength (- (Math|Transform|TransformLocation (Transformation|GetRelativeTransform (Utilities|Array|Get(acopy) _spawned_utility_pole_reference_4 (- _index 1))) (.location (Variables|PowerlineLocation|GetPowerline%203A))) (Math|Transform|TransformLocation (Transformation|GetRelativeTransform (Utilities|Array|Get(acopy) _spawned_utility_pole_reference_4 (select (== _index (Variables|Default|GetCount%20per%20spline)) 0 _index))) (.location (Variables|PowerlineLocation|GetPowerline%203B)))))) (Math|Vector|MakeVector 0.0 0.0 _returnvalue)) true :!class /Script/Engine.SplineMeshComponent)
          (SplineMesh|SetStartScale _returnvalue_17 (Math|Vector2D|MakeVector2D _powerline_size_4 _powerline_size_4) true :!class /Script/Engine.SplineMeshComponent)
          (SplineMesh|SetEndScale _returnvalue_17 (Math|Vector2D|MakeVector2D _powerline_size_4 _powerline_size_4) true :!class /Script/Engine.SplineMeshComponent)))
      (:then_3
        (if (Variables|Default|GetUse%20Powerline%204?)
          (bind _returnvalue_18 (AddComponent|AddSplineMeshComponent false))
          (Components|StaticMesh|SetStaticMesh _returnvalue_18 (Variables|Default|GetNew%20Cable%20Mesh))
          (SplineMesh|SetStartandEnd _returnvalue_18 (Math|Transform|TransformLocation (Transformation|GetRelativeTransform (Utilities|Array|Get(acopy) _spawned_utility_pole_reference_5 (- _index 1))) (.location (Variables|PowerlineLocation|GetPowerline%204A))) (- (* (Math|Rotator|GetRotationXVector (Math|Rotator|FindLookatRotation (Math|Transform|TransformLocation (Transformation|GetRelativeTransform (Utilities|Array|Get(acopy) _spawned_utility_pole_reference_5 (- _index 1))) (.location (Variables|PowerlineLocation|GetPowerline%204A))) (Math|Transform|TransformLocation (Transformation|GetRelativeTransform (Utilities|Array|Get(acopy) _spawned_utility_pole_reference_5 (select (== _index (Variables|Default|GetCount%20per%20spline)) 0 _index))) (.location (Variables|PowerlineLocation|GetPowerline%204B))))) (Math|Vector|VectorLength (- (Math|Transform|TransformLocation (Transformation|GetRelativeTransform (Utilities|Array|Get(acopy) _spawned_utility_pole_reference_5 (- _index 1))) (.location (Variables|PowerlineLocation|GetPowerline%204A))) (Math|Transform|TransformLocation (Transformation|GetRelativeTransform (Utilities|Array|Get(acopy) _spawned_utility_pole_reference_5 (select (== _index (Variables|Default|GetCount%20per%20spline)) 0 _index))) (.location (Variables|PowerlineLocation|GetPowerline%204B)))))) (Math|Vector|MakeVector 0.0 0.0 _returnvalue_2)) (Math|Transform|TransformLocation (Transformation|GetRelativeTransform (Utilities|Array|Get(acopy) _spawned_utility_pole_reference_5 (select (== _index (Variables|Default|GetCount%20per%20spline)) 0 _index))) (.location (Variables|PowerlineLocation|GetPowerline%204B))) (+ (* (Math|Rotator|GetRotationXVector (Math|Rotator|FindLookatRotation (Math|Transform|TransformLocation (Transformation|GetRelativeTransform (Utilities|Array|Get(acopy) _spawned_utility_pole_reference_5 (- _index 1))) (.location (Variables|PowerlineLocation|GetPowerline%204A))) (Math|Transform|TransformLocation (Transformation|GetRelativeTransform (Utilities|Array|Get(acopy) _spawned_utility_pole_reference_5 (select (== _index (Variables|Default|GetCount%20per%20spline)) 0 _index))) (.location (Variables|PowerlineLocation|GetPowerline%204B))))) (Math|Vector|VectorLength (- (Math|Transform|TransformLocation (Transformation|GetRelativeTransform (Utilities|Array|Get(acopy) _spawned_utility_pole_reference_5 (- _index 1))) (.location (Variables|PowerlineLocation|GetPowerline%204A))) (Math|Transform|TransformLocation (Transformation|GetRelativeTransform (Utilities|Array|Get(acopy) _spawned_utility_pole_reference_5 (select (== _index (Variables|Default|GetCount%20per%20spline)) 0 _index))) (.location (Variables|PowerlineLocation|GetPowerline%204B)))))) (Math|Vector|MakeVector 0.0 0.0 _returnvalue_2)) true :!class /Script/Engine.SplineMeshComponent)
          (SplineMesh|SetStartScale _returnvalue_18 (Math|Vector2D|MakeVector2D _powerline_size_5 _powerline_size_5) true :!class /Script/Engine.SplineMeshComponent)
          (SplineMesh|SetEndScale _returnvalue_18 (Math|Vector2D|MakeVector2D _powerline_size_5 _powerline_size_5) true :!class /Script/Engine.SplineMeshComponent)))
      (:then_4
        (if (Variables|Default|GetUse%20Powerline%205?)
          (bind _returnvalue_19 (AddComponent|AddSplineMeshComponent false))
          (Components|StaticMesh|SetStaticMesh _returnvalue_19 (Variables|Default|GetNew%20Cable%20Mesh))
          (SplineMesh|SetStartandEnd _returnvalue_19 (Math|Transform|TransformLocation (Transformation|GetRelativeTransform (Utilities|Array|Get(acopy) _spawned_utility_pole_reference_6 (- _index 1))) (.location (Variables|PowerlineLocation|GetPowerline%205A))) (- (* (Math|Rotator|GetRotationXVector (Math|Rotator|FindLookatRotation (Math|Transform|TransformLocation (Transformation|GetRelativeTransform (Utilities|Array|Get(acopy) _spawned_utility_pole_reference_6 (- _index 1))) (.location (Variables|PowerlineLocation|GetPowerline%205A))) (Math|Transform|TransformLocation (Transformation|GetRelativeTransform (Utilities|Array|Get(acopy) _spawned_utility_pole_reference_6 (select (== _index (Variables|Default|GetCount%20per%20spline)) 0 _index))) (.location (Variables|PowerlineLocation|GetPowerline%205B))))) (Math|Vector|VectorLength (- (Math|Transform|TransformLocation (Transformation|GetRelativeTransform (Utilities|Array|Get(acopy) _spawned_utility_pole_reference_6 (- _index 1))) (.location (Variables|PowerlineLocation|GetPowerline%205A))) (Math|Transform|TransformLocation (Transformation|GetRelativeTransform (Utilities|Array|Get(acopy) _spawned_utility_pole_reference_6 (select (== _index (Variables|Default|GetCount%20per%20spline)) 0 _index))) (.location (Variables|PowerlineLocation|GetPowerline%205B)))))) (Math|Vector|MakeVector 0.0 0.0 _returnvalue_3)) (Math|Transform|TransformLocation (Transformation|GetRelativeTransform (Utilities|Array|Get(acopy) _spawned_utility_pole_reference_6 (select (== _index (Variables|Default|GetCount%20per%20spline)) 0 _index))) (.location (Variables|PowerlineLocation|GetPowerline%205B))) (+ (* (Math|Rotator|GetRotationXVector (Math|Rotator|FindLookatRotation (Math|Transform|TransformLocation (Transformation|GetRelativeTransform (Utilities|Array|Get(acopy) _spawned_utility_pole_reference_6 (- _index 1))) (.location (Variables|PowerlineLocation|GetPowerline%205A))) (Math|Transform|TransformLocation (Transformation|GetRelativeTransform (Utilities|Array|Get(acopy) _spawned_utility_pole_reference_6 (select (== _index (Variables|Default|GetCount%20per%20spline)) 0 _index))) (.location (Variables|PowerlineLocation|GetPowerline%205B))))) (Math|Vector|VectorLength (- (Math|Transform|TransformLocation (Transformation|GetRelativeTransform (Utilities|Array|Get(acopy) _spawned_utility_pole_reference_6 (- _index 1))) (.location (Variables|PowerlineLocation|GetPowerline%205A))) (Math|Transform|TransformLocation (Transformation|GetRelativeTransform (Utilities|Array|Get(acopy) _spawned_utility_pole_reference_6 (select (== _index (Variables|Default|GetCount%20per%20spline)) 0 _index))) (.location (Variables|PowerlineLocation|GetPowerline%205B)))))) (Math|Vector|MakeVector 0.0 0.0 _returnvalue_3)) true :!class /Script/Engine.SplineMeshComponent)
          (SplineMesh|SetStartScale _returnvalue_19 (Math|Vector2D|MakeVector2D _powerline_size_6 _powerline_size_6) true :!class /Script/Engine.SplineMeshComponent)
          (SplineMesh|SetEndScale _returnvalue_19 (Math|Vector2D|MakeVector2D _powerline_size_6 _powerline_size_6) true :!class /Script/Engine.SplineMeshComponent)))
      (:then_5
        (if (Variables|Default|GetUse%20Powerline%206?)
          (bind _returnvalue_20 (AddComponent|AddSplineMeshComponent false))
          (Components|StaticMesh|SetStaticMesh _returnvalue_20 (Variables|Default|GetNew%20Cable%20Mesh))
          (SplineMesh|SetStartandEnd _returnvalue_20 (Math|Transform|TransformLocation (Transformation|GetRelativeTransform (Utilities|Array|Get(acopy) _spawned_utility_pole_reference (- _index 1))) (.location (Variables|PowerlineLocation|GetPowerline%206A))) (- (* (Math|Rotator|GetRotationXVector (Math|Rotator|FindLookatRotation (Math|Transform|TransformLocation (Transformation|GetRelativeTransform (Utilities|Array|Get(acopy) _spawned_utility_pole_reference (- _index 1))) (.location (Variables|PowerlineLocation|GetPowerline%206A))) (Math|Transform|TransformLocation (Transformation|GetRelativeTransform (Utilities|Array|Get(acopy) _spawned_utility_pole_reference (select (== _index (Variables|Default|GetCount%20per%20spline)) 0 _index))) (.location (Variables|PowerlineLocation|GetPowerline%206B))))) (Math|Vector|VectorLength (- (Math|Transform|TransformLocation (Transformation|GetRelativeTransform (Utilities|Array|Get(acopy) _spawned_utility_pole_reference (- _index 1))) (.location (Variables|PowerlineLocation|GetPowerline%206A))) (Math|Transform|TransformLocation (Transformation|GetRelativeTransform (Utilities|Array|Get(acopy) _spawned_utility_pole_reference (select (== _index (Variables|Default|GetCount%20per%20spline)) 0 _index))) (.location (Variables|PowerlineLocation|GetPowerline%206B)))))) (Math|Vector|MakeVector 0.0 0.0 _returnvalue_6)) (Math|Transform|TransformLocation (Transformation|GetRelativeTransform (Utilities|Array|Get(acopy) _spawned_utility_pole_reference (select (== _index (Variables|Default|GetCount%20per%20spline)) 0 _index))) (.location (Variables|PowerlineLocation|GetPowerline%206B))) (+ (* (Math|Rotator|GetRotationXVector (Math|Rotator|FindLookatRotation (Math|Transform|TransformLocation (Transformation|GetRelativeTransform (Utilities|Array|Get(acopy) _spawned_utility_pole_reference (- _index 1))) (.location (Variables|PowerlineLocation|GetPowerline%206A))) (Math|Transform|TransformLocation (Transformation|GetRelativeTransform (Utilities|Array|Get(acopy) _spawned_utility_pole_reference (select (== _index (Variables|Default|GetCount%20per%20spline)) 0 _index))) (.location (Variables|PowerlineLocation|GetPowerline%206B))))) (Math|Vector|VectorLength (- (Math|Transform|TransformLocation (Transformation|GetRelativeTransform (Utilities|Array|Get(acopy) _spawned_utility_pole_reference (- _index 1))) (.location (Variables|PowerlineLocation|GetPowerline%206A))) (Math|Transform|TransformLocation (Transformation|GetRelativeTransform (Utilities|Array|Get(acopy) _spawned_utility_pole_reference (select (== _index (Variables|Default|GetCount%20per%20spline)) 0 _index))) (.location (Variables|PowerlineLocation|GetPowerline%206B)))))) (Math|Vector|MakeVector 0.0 0.0 _returnvalue_6)) true :!class /Script/Engine.SplineMeshComponent)
          (SplineMesh|SetStartScale _returnvalue_20 (Math|Vector2D|MakeVector2D _powerline_size _powerline_size) true :!class /Script/Engine.SplineMeshComponent)
          (SplineMesh|SetEndScale _returnvalue_20 (Math|Vector2D|MakeVector2D _powerline_size _powerline_size) true :!class /Script/Engine.SplineMeshComponent))))))
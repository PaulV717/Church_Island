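; BP_Blockout is a level blockout actor that shows either a box or a ramp mesh, chosen by ObjectType.
; All logic runs in the construction script, which scales the mesh from CornerLocation divided by 100 to size the shape.
; It applies CustomMaterial if valid, otherwise creates a dynamic instance of M_WorldProject driven by colour, top-colour, texture-size and roughness variables.
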(event EventBeginPlay)

(event Collision|EventActorBeginOverlap
  (params (OtherActor :type Actor%20Object%20Reference)))

(event EventTick
  (params (DeltaSeconds :type Float%20%28single-precision%29)))

(fn ConstructionScript
  (bind _corner_location (Variables|Default|GetCorner%20Location))
  (bind _returnvalue (/ _corner_location 1e+02))
  (Components|StaticMesh|SetStaticMesh (Variables|Default|GetBox_Corner) (Utilities|Select :Index (Variables|Default|GetObject%20Type) :NewEnumerator0 "/Game/Blockout/Geometry/Foundational/SM_Box_Corner.SM_Box_Corner" :NewEnumerator1 "/Game/Blockout/Geometry/Foundational/SM_Ramp_1.SM_Ramp_1"))
  (Transformation|SetRelativeScale3D (Variables|Default|GetBox_Corner) (Math|Vector|MakeVector (.x _returnvalue) (.y _returnvalue) (.z _returnvalue)))
  (Utilities|IsValid (Variables|Default|GetCustom%20Material)
    (:Is%20Valid
      (Rendering|Material|SetMaterial (Variables|Default|GetBox_Corner) 0 (Variables|Default|GetCustom%20Material)))
    (:Is%20Not%20Valid
      (bind _returnvalue_2 (Rendering|Material|CreateDynamicMaterialInstance "/Game/Blockout/Material/Base/M_WorldProject.M_WorldProject" "None" :!class /Script/Engine.KismetMaterialLibrary))
      (Rendering|Material|SetMaterial (Variables|Default|GetBox_Corner) 0 _returnvalue_2)
      (Rendering|Material|SetVectorParameterValue _returnvalue_2 "Diffuse Colour" (Variables|Default|GetSurface%20Colour) :!class /Script/Engine.MaterialInstanceDynamic)
      (Rendering|Material|SetScalarParameterValue _returnvalue_2 "Unique colour for top?" (Math|Conversions|ToFloat(Boolean) (Variables|Default|GetUnique%20colour%20for%20top?)) :!class /Script/Engine.MaterialInstanceDynamic)
      (Rendering|Material|SetVectorParameterValue _returnvalue_2 "Diffuse Colour - Top" (Variables|Default|GetTop%20Colour) :!class /Script/Engine.MaterialInstanceDynamic)
      (Rendering|Material|SetScalarParameterValue _returnvalue_2 "Multiply texture size" (Math|Conversions|ToFloat(Integer) (Variables|Default|GetMultiply%20texture%20size)) :!class /Script/Engine.MaterialInstanceDynamic)
      (Rendering|Material|SetScalarParameterValue _returnvalue_2 "Roughness" (Variables|Default|GetMaterial%20Roughness%20Value) :!class /Script/Engine.MaterialInstanceDynamic))))
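; Blockout actor that builds a selectable primitive shape, such as a box, cylinder, sphere, cone, pyramid or bevel, in its construction script.
; ObjectType picks the static mesh, Radius sets its X and Y scale, and CornerLocation, locked to the vertical axis, sets its height.
; A valid custom material takes priority; otherwise an optional dynamic debug material applies surface colour, separate top colour and roughness.
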(event EventBeginPlay)

(event Collision|EventActorBeginOverlap
  (params (OtherActor :type Actor%20Object%20Reference)))

(event EventTick
  (params (DeltaSeconds :type Float%20%28single-precision%29)))

(fn ConstructionScript
  (bind _radius (Variables|Default|GetRadius))
  (bind _returnvalue (/ _radius 1e+02))
  (Variables|Default|SetCorner%20Location (Math|Vector|MakeVector 0.0 0.0 (.z (Variables|Default|GetCorner%20Location))))
  (Components|StaticMesh|SetStaticMesh (Variables|Default|GetObject) (Utilities|Select :Index (Variables|Default|GetObject%20Type) :NewEnumerator0 "/Game/Blockout/Geometry/Foundational/SM_Box_Bottom.SM_Box_Bottom" :NewEnumerator1 "/Game/Blockout/Geometry/Foundational/SM_Cylinder_Bottom.SM_Cylinder_Bottom" :NewEnumerator8 "/Game/Blockout/Geometry/Foundational/SM_QuarterCylinder.SM_QuarterCylinder" :NewEnumerator2 "/Game/Blockout/Geometry/Foundational/SM_Sphere_Center.SM_Sphere_Center" :NewEnumerator3 "/Game/Blockout/Geometry/Foundational/SM_Sphere_Base.SM_Sphere_Base" :NewEnumerator4 "/Game/Blockout/Geometry/Foundational/SM_Cone_Bottom.SM_Cone_Bottom" :NewEnumerator5 "/Game/Blockout/Geometry/Foundational/SM_Pyramid_Base.SM_Pyramid_Base" :NewEnumerator7 "/Game/Blockout/Geometry/Foundational/SM_Corner_Bevel.SM_Corner_Bevel" :NewEnumerator9 "/Game/Blockout/Geometry/Foundational/SM_Pyramid_Triangular.SM_Pyramid_Triangular" :NewEnumerator10 "/Game/Blockout/Geometry/Foundational/SM_Pyramid_Triangular_End.SM_Pyramid_Triangular_End"))
  (Transformation|SetRelativeScale3D (Variables|Default|GetObject) (Math|Vector|MakeVector _returnvalue _returnvalue (.z (/ (Variables|Default|GetCorner%20Location) 1e+02))))
  (Utilities|IsValid (Variables|Material|GetCustom%20Material)
    (:Is%20Valid
      (Rendering|Material|SetMaterial (Variables|Default|GetObject) (Variables|Material|GetCustom%20Material%20ID) (Variables|Material|GetCustom%20Material)))
    (:Is%20Not%20Valid
      (if (Variables|Material|GetUse%20Debug%20Material?)
        (bind _returnvalue_2 (Rendering|Material|CreateDynamicMaterialInstance "/Game/Blockout/Material/Base/M_WorldProject.M_WorldProject" "None" :!class /Script/Engine.KismetMaterialLibrary))
        (Rendering|Material|SetMaterial (Variables|Default|GetObject) 0 _returnvalue_2)
        (Rendering|Material|SetVectorParameterValue _returnvalue_2 "Diffuse Colour" (Variables|Material|GetSurface%20Colour) :!class /Script/Engine.MaterialInstanceDynamic)
        (Rendering|Material|SetScalarParameterValue _returnvalue_2 "Unique colour for top?" (Math|Conversions|ToFloat(Boolean) (Variables|Material|GetUnique%20colour%20for%20top?)) :!class /Script/Engine.MaterialInstanceDynamic)
        (Rendering|Material|SetVectorParameterValue _returnvalue_2 "Diffuse Colour - Top" (Variables|Material|GetTop%20Colour) :!class /Script/Engine.MaterialInstanceDynamic)
        (Rendering|Material|SetScalarParameterValue _returnvalue_2 "Roughness" (Variables|Material|GetMaterial%20Roughness%20Value) :!class /Script/Engine.MaterialInstanceDynamic)))))
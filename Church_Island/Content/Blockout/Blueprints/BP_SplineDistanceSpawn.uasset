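; Blockout spline actor whose construction script places copies of a static mesh at even distances along its spline.
; Placement uses either a fixed spacing or a count per spline, with the count's step adjusted for closed loops.
; Each copy is a separate mesh component following the spline's full tangent rotation or only its yaw, plus a yaw offset.
; A custom material takes priority over an optional tinted debug dynamic material.
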(event EventBeginPlay)

(event Collision|EventActorBeginOverlap
  (params (OtherActor :type Actor%20Object%20Reference)))

(event EventTick
  (params (DeltaSeconds :type Float%20%28single-precision%29)))

(fn ConstructionScript
  (bind _spline (Variables|Default|GetSpline))
  (bind _custom_material (Variables|Material|GetCustom%20Material))
  (bind _count_per_spline (Variables|Default|GetCount%20per%20spline))
  (Spline|SetClosedLoop (Variables|Default|GetSpline) (Variables|Default|GetIs%20Closed%20loop?) true)
  (Variables|Variables|SetSpline%20Length (Spline|GetSplineLength (Variables|Default|GetSpline)))
  (Utilities|IsValid (Variables|Material|GetCustom%20Material)
    (:Is%20Valid
      _)
    (:Is%20Not%20Valid
      (if (Variables|Material|GetUse%20Debug%20Material?)
        (bind _returnvalue (Rendering|Material|CreateDynamicMaterialInstance "/Game/Blockout/Material/Base/M_WorldProject.M_WorldProject" "None" :!class /Script/Engine.KismetMaterialLibrary))
        (bind _output_get (Variables|Variables|SetDynamic%20Material _returnvalue))
        (Rendering|Material|SetVectorParameterValue _output_get "Diffuse Colour" (Variables|Material|GetSurface%20Colour) :!class /Script/Engine.MaterialInstanceDynamic)
        (Rendering|Material|SetScalarParameterValue _output_get "Unique colour for top?" (Math|Conversions|ToFloat(Boolean) (Variables|Default|GetUnique%20colour%20for%20top?)) :!class /Script/Engine.MaterialInstanceDynamic)
        (Rendering|Material|SetVectorParameterValue _output_get "Diffuse Colour - Top" (Variables|Material|GetTop%20Colour) :!class /Script/Engine.MaterialInstanceDynamic)
        (Rendering|Material|SetScalarParameterValue _output_get "Roughness" (Variables|Material|GetMaterial%20Roughness%20Value) :!class /Script/Engine.MaterialInstanceDynamic))))
  (for _index (range 0 (select (Variables|Default|GetT-Spacing%20F-Count%20per%20spline) (Math|Float|Floor (/ (Variables|Variables|GetSpline%20Length) (Variables|Default|GetSpacing))) (- (Variables|Default|GetCount%20per%20spline) 1)))
    (bind _returnvalue_2 (AddComponent|AddStaticMeshComponent false (Math|Transform|MakeTransform (Spline|GetLocationatDistanceAlongSpline _spline (* _index (select (Variables|Default|GetT-Spacing%20F-Count%20per%20spline) (Variables|Default|GetSpacing) (/ (Variables|Variables|GetSpline%20Length) (Math|Conversions|ToFloat(Integer) (select (Variables|Default|GetIs%20Closed%20loop?) (- _count_per_spline 0) (- _count_per_spline 1)))))) "Local") (select (Variables|Default|GetAlign%20to%20splines%20orientation?) (Math|Conversions|RotationFromXVector (Spline|GetTangentatDistanceAlongSpline _spline (* _index (select (Variables|Default|GetT-Spacing%20F-Count%20per%20spline) (Variables|Default|GetSpacing) (/ (Variables|Variables|GetSpline%20Length) (Math|Conversions|ToFloat(Integer) (select (Variables|Default|GetIs%20Closed%20loop?) (- _count_per_spline 0) (- _count_per_spline 1)))))) "Local")) (Math|Rotator|MakeRotator 0.0 0.0 (.Yaw (Math|Rotator|BreakRotator (Math|Conversions|RotationFromXVector (Spline|GetTangentatDistanceAlongSpline _spline (* _index (select (Variables|Default|GetT-Spacing%20F-Count%20per%20spline) (Variables|Default|GetSpacing) (/ (Variables|Variables|GetSpline%20Length) (Math|Conversions|ToFloat(Integer) (select (Variables|Default|GetIs%20Closed%20loop?) (- _count_per_spline 0) (- _count_per_spline 1)))))) "Local")))))) (Variables|Default|GetAsset%20Scale))))
    (Components|StaticMesh|SetStaticMesh _returnvalue_2 (Variables|Default|GetNew%20Static%20Mesh))
    (Transformation|AddLocalRotation _returnvalue_2 (Math|Rotator|MakeRotator 0.0 0.0 (Variables|Default|GetRotate%20Assets)) false false)
    (Utilities|IsValid _custom_material
      (:Is%20Valid
        (Rendering|Material|SetMaterial _returnvalue_2 (Variables|Material|GetCustom%20Material%20ID) _custom_material))
      (:Is%20Not%20Valid
        (if (Variables|Material|GetUse%20Debug%20Material?)
          (Rendering|Material|SetMaterial _returnvalue_2 0 (Variables|Variables|GetDynamic%20Material)))))))
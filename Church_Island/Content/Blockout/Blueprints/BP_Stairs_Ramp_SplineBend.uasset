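; Blockout construction-script actor that builds a curved staircase or ramp, with optional foundation, bent toward the StairDestination transform.
; A two-point spline follows the destination's XY and yaw, with X scale driving tangent strength and Y scale the width.
; One spline mesh, chosen from four variants by spline length, is Z-scaled to the destination height.
; It takes a custom material or a tinted M_WorldProject dynamic instance.
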(event EventBeginPlay)

(event Collision|EventActorBeginOverlap
  (params (OtherActor :type Actor%20Object%20Reference)))

(event EventTick
  (params (DeltaSeconds :type Float%20%28single-precision%29)))

(fn ConstructionScript
  (bind _spline (Variables|Default|GetSpline))
  (bind _spline_2 (Variables|Default|GetSpline))
  (bind _spline_3 (Variables|Default|GetSpline))
  (bind _spline_4 (Variables|Default|GetSpline))
  (bind _returnvalue (Spline|GetSplineLength _spline_2))
  (bind _returnvalue_2 (Spline|GetSplineLength _spline_3))
  (bind _returnvalue_3 (- _returnvalue_2 5e+01))
  (bind _returnvalue_4 (* _returnvalue 2.5))
  (bind _returnvalue_5 (/ _returnvalue_3 2.5e+02))
  (bind _returnvalue_6 (Math|Float|Floor _returnvalue_5))
  (bind _returnvalue_7 (Math|Integer|Clamp(Integer) _returnvalue_6 0 3))
  (Utilities|Array|Clear (Variables|Variables|GetCreated%20Assets%20%28Reference%29))
  (Variables|Default|SetStair%20Destination (Math|Transform|MakeTransform (.location (Variables|Default|GetStair%20Destination)) (Math|Rotator|MakeRotator 0.0 0.0 (.yaw (.rotation (Variables|Default|GetStair%20Destination)))) (.scale (Variables|Default|GetStair%20Destination))))
  (Spline|SetLocationatSplinePoint (Variables|Default|GetSpline) 0 (Math|Vector|MakeVector 0.0 0.0 0.0) "Local" false)
  (Spline|SetTangentatSplinePoint (Variables|Default|GetSpline) 0 (* "1.000000, 0, 0" (* (.x (.scale (Variables|Default|GetStair%20Destination))) _returnvalue_4)) "Local" false)
  (Spline|SetLocationatSplinePoint (Variables|Default|GetSpline) 1 (Math|Vector|MakeVector (.x (.location (Variables|Default|GetStair%20Destination))) (.y (.location (Variables|Default|GetStair%20Destination))) 0.0) "Local" false)
  (Spline|SetTangentatSplinePoint (Variables|Default|GetSpline) 1 (* (Math|Vector|GetForwardVector (.rotation (Variables|Default|GetStair%20Destination))) (* (.x (.scale (Variables|Default|GetStair%20Destination))) _returnvalue_4)) "Local" true)
  (Variables|Default|SetNew%20Spline%20Asset (select (Variables|Default|GetUse%20Stairs?) (select (Variables|Default|GetUse%20Foundation?) (Utilities|Select :Index _returnvalue_7 :Option%200 "/Game/Blockout/Geometry/Foundational/Spline/SM_Stairs_1_Base_Spline.SM_Stairs_1_Base_Spline" :Option%201 "/Game/Blockout/Geometry/Foundational/Spline/SM_Stairs_2_Base_Spline.SM_Stairs_2_Base_Spline" :Option%202 "/Game/Blockout/Geometry/Foundational/Spline/SM_Stairs_3_Base_Spline.SM_Stairs_3_Base_Spline" :Option%203 "/Game/Blockout/Geometry/Foundational/Spline/SM_Stairs_4_Base_Spline.SM_Stairs_4_Base_Spline") (Utilities|Select :Index _returnvalue_7 :Option%200 "/Game/Blockout/Geometry/Foundational/Spline/SM_Stairs_1_Spline.SM_Stairs_1_Spline" :Option%201 "/Game/Blockout/Geometry/Foundational/Spline/SM_Stairs_2_Spline.SM_Stairs_2_Spline" :Option%202 "/Game/Blockout/Geometry/Foundational/Spline/SM_Stairs_3_Spline.SM_Stairs_3_Spline" :Option%203 "/Game/Blockout/Geometry/Foundational/Spline/SM_Stairs_4_Spline.SM_Stairs_4_Spline")) (select (Variables|Default|GetUse%20Foundation?) (Utilities|Select :Index _returnvalue_7 :Option%200 "/Game/Blockout/Geometry/Foundational/Spline/SM_Ramp_A1_Spline.SM_Ramp_A1_Spline" :Option%201 "/Game/Blockout/Geometry/Foundational/Spline/SM_Ramp_A2_Spline.SM_Ramp_A2_Spline" :Option%202 "/Game/Blockout/Geometry/Foundational/Spline/SM_Ramp_A3_Spline.SM_Ramp_A3_Spline" :Option%203 "/Game/Blockout/Geometry/Foundational/Spline/SM_Ramp_A4_Spline.SM_Ramp_A4_Spline") (Utilities|Select :Index _returnvalue_7 :Option%200 "/Game/Blockout/Geometry/Foundational/Spline/SM_Ramp_B1_Spline.SM_Ramp_B1_Spline" :Option%201 "/Game/Blockout/Geometry/Foundational/Spline/SM_Ramp_B2_Spline.SM_Ramp_B2_Spline" :Option%202 "/Game/Blockout/Geometry/Foundational/Spline/SM_Ramp_B3_Spline.SM_Ramp_B3_Spline" :Option%203 "/Game/Blockout/Geometry/Foundational/Spline/SM_Ramp_B4_Spline.SM_Ramp_B4_Spline"))))
  (bind _returnvalue_8 (AddComponent|AddSplineMeshComponent false (Math|Transform|MakeTransform "0, 0, 0" "0, 0, 0" (Math|Vector|MakeVector 1.0 1.0 (/ (.z (.location (Variables|Default|GetStair%20Destination))) (- (.z (.max (StaticMesh|GetBoundingBox (Variables|Default|GetNew%20Spline%20Asset)))) (.z (.min (StaticMesh|GetBoundingBox (Variables|Default|GetNew%20Spline%20Asset))))))))))
  (Utilities|Array|Add (Variables|Variables|GetCreated%20Assets%20%28Reference%29) _returnvalue_8)
  (SplineMesh|SetForwardAxis _returnvalue_8 (Variables|Default|GetForward%20Axis) true)
  (Components|StaticMesh|SetStaticMesh _returnvalue_8 (Variables|Default|GetNew%20Spline%20Asset))
  (SplineMesh|SetStartandEnd _returnvalue_8 (Spline|GetLocationatSplinePoint _spline 0 "Local") (Spline|GetTangentatSplinePoint _spline 0 "Local") (Spline|GetLocationatSplinePoint _spline_4 1 "Local") (Spline|GetTangentatSplinePoint _spline_4 1 "Local") true :!class /Script/Engine.SplineMeshComponent)
  (SplineMesh|SetStartScale _returnvalue_8 (Math|Vector2D|MakeVector2D (.y (.scale (Variables|Default|GetStair%20Destination))) 1.0) true :!class /Script/Engine.SplineMeshComponent)
  (SplineMesh|SetEndScale _returnvalue_8 (Math|Vector2D|MakeVector2D (.y (.scale (Variables|Default|GetStair%20Destination))) 1.0) true :!class /Script/Engine.SplineMeshComponent)
  (Utilities|IsValid (Variables|Material|GetCustom%20Material)
    (:Is%20Valid
      (Rendering|Material|SetMaterial _returnvalue_8 0 (Variables|Material|GetCustom%20Material)))
    (:Is%20Not%20Valid
      (bind _returnvalue_9 (Rendering|Material|CreateDynamicMaterialInstance "/Game/Blockout/Material/Base/M_WorldProject.M_WorldProject" "None" :!class /Script/Engine.KismetMaterialLibrary))
      (Rendering|Material|SetMaterial _returnvalue_8 0 _returnvalue_9)
      (Rendering|Material|SetVectorParameterValue _returnvalue_9 "Diffuse Colour" (Variables|Material|GetSurface%20Colour) :!class /Script/Engine.MaterialInstanceDynamic)
      (Rendering|Material|SetScalarParameterValue _returnvalue_9 "Unique colour for top?" (Math|Conversions|ToFloat(Boolean) (Variables|Default|GetUnique%20colour%20for%20top?)) :!class /Script/Engine.MaterialInstanceDynamic)
      (Rendering|Material|SetVectorParameterValue _returnvalue_9 "Diffuse Colour - Top" (Variables|Material|GetTop%20Colour) :!class /Script/Engine.MaterialInstanceDynamic)
      (Rendering|Material|SetScalarParameterValue _returnvalue_9 "Roughness" (Variables|Material|GetMaterial%20Roughness%20Value) :!class /Script/Engine.MaterialInstanceDynamic))))
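; Two-stop elevator, vertical or inclined, operated by top and bottom call buttons or E while the player stands in its box.
; A timeline lerps the floor hinge along ElevatorHeight; calls made mid-travel are remembered, triggering a return after a pause.
; Finished moves and redundant calls reset BP_Button colours.
; The construction script applies meshes, places buttons, fits the box, scales and tilts the guide, and counter-rotates the floor to stay level.
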(event OnComponentBeginOverlap(Box)
  (params (OverlappedComponent :type Primitive%20Component%20Object%20Reference) (OtherActor :type Actor%20Object%20Reference) (OtherComp :type Primitive%20Component%20Object%20Reference) (OtherBodyIndex :type Integer) (bFromSweep :type Boolean) (SweepResult :type Hit%20Result%20Structure%20%28by%20ref%29))
  (if (== OtherActor (Game|Player|GetPlayerPawn 0))
    (Input|EnableInput (Game|GetPlayerController 0))))

(event OnComponentEndOverlap(Box)
  (params (OverlappedComponent :type Primitive%20Component%20Object%20Reference) (OtherActor :type Actor%20Object%20Reference) (OtherComp :type Primitive%20Component%20Object%20Reference) (OtherBodyIndex :type Integer))
  (if (== OtherActor (Game|Player|GetPlayerPawn 0))
    (Input|DisableInput (Game|GetPlayerController 0))))

(event Custom|Call%20button%20was%20pressed
  (params (Location :type String))
  (bind _animate_up_down (Variables|Default|GetAnimate%20Up/Down))
  (bind _is_delay_activated_before_returning_ (Variables|Variables|GetIs%20delay%20activated%20before%20returning?))
  (bind _returnvalue (Audio|Components|Audio|IsPlaying _animate_up_down))
  (Utilities|FlowControl|Sequence
    (:then_0
      (if (Utilities|Enum|Equal(Enum) Location "Top")
        (if _returnvalue
          (Variables|Variables|SetTop%20call%20button%20was%20pressed? true)
          (elif (Variables|Default|GetIs%20the%20elevator%20at%20the%20top?)
            (Utilities|FlowControl|Delay 0.5)
            (bind _asbp_button (Utilities|Casting|CastToBP_Button (Variables|/Script/Engine.ChildActorComponent|GetChildActor (Variables|Default|GetButton_Top_BP))))
            (Default|ReturnMaterialtoDefaultColour _asbp_button)
            (elif (not _is_delay_activated_before_returning_)
              (CallFunction|TriggerElevator :!label _label))))))
    (:then_1
      (if (Utilities|Enum|Equal(Enum) Location "Bottom")
        (if _returnvalue
          (Variables|Variables|SetBottom%20call%20button%20was%20pressed? true)
          (elif (Variables|Default|GetIs%20the%20elevator%20at%20the%20top?)
            (if (not _is_delay_activated_before_returning_)
              (goto _label))
            (else
              (Utilities|FlowControl|Delay 0.5)
              (bind _asbp_button_2 (Utilities|Casting|CastToBP_Button (Variables|/Script/Engine.ChildActorComponent|GetChildActor (Variables|Default|GetButton_Bottom_BP))))
              (Default|ReturnMaterialtoDefaultColour _asbp_button_2))))))))

(event Custom|Trigger%20Elevator
  (if (not (Variables|Variables|GetIs%20delay%20activated%20before%20returning?))
    (if (Variables|Default|GetIs%20the%20elevator%20at%20the%20top?)
      (Variables|Default|SetIs%20the%20elevator%20at%20the%20top? false)
      (bind (_direction _0_1) (Timeline|Animate%20Up/Down ReverseFromEnd)
        (:Update
          (Transformation|SetRelativeLocation (Variables|Default|GetElevator_FloorHinge) (Math|Vector|Lerp(Vector) "0, 0, 0" (Variables|Default|GetElevator%20Height) _0_1) false true))
        (:Finished
          (switch Utilities|FlowControl|Switch|SwitchonETimelineDirection _direction
            (:Forward
              (bind _asbp_button (Utilities|Casting|CastToBP_Button (Variables|/Script/Engine.ChildActorComponent|GetChildActor (Variables|Default|GetButton_Top_BP))))
              (Default|ReturnMaterialtoDefaultColour _asbp_button)
              (if (Variables|Variables|GetBottom%20call%20button%20was%20pressed?)
                (Variables|Variables|SetBottom%20call%20button%20was%20pressed? false)
                (Variables|Variables|SetIs%20delay%20activated%20before%20returning? true)
                (Utilities|FlowControl|Delay (Variables|Default|GetFloor%20pause%20time%20before%20returning%20when%20called) :!label _label)
                (Variables|Variables|SetIs%20delay%20activated%20before%20returning? false)
                (CallFunction|TriggerElevator)))
            (:Backward
              (bind _asbp_button_2 (Utilities|Casting|CastToBP_Button (Variables|/Script/Engine.ChildActorComponent|GetChildActor (Variables|Default|GetButton_Bottom_BP))))
              (Default|ReturnMaterialtoDefaultColour _asbp_button_2)
              (if (Variables|Variables|GetTop%20call%20button%20was%20pressed?)
                (Variables|Variables|SetTop%20call%20button%20was%20pressed? false)
                (Variables|Variables|SetIs%20delay%20activated%20before%20returning? true)
                (goto _label))))))
      (else
        (Variables|Default|SetIs%20the%20elevator%20at%20the%20top? true)
        (Timeline|Animate%20Up/Down PlayFromStart)))))

(event EventBeginPlay
  (Components|Timeline|SetPlayRate (Variables|Default|GetAnimate%20Up/Down) (/ 1.0 (Variables|Default|GetLength%20of%20time%20it%20takes%20to%20travel))))

(event Input|KeyboardEvents|E
  (params (Key :type Key%20Structure))
  (:Pressed
    (if (not (Audio|Components|Audio|IsPlaying (Variables|Default|GetAnimate%20Up/Down)))
      (if (not (Variables|Variables|GetIs%20delay%20activated%20before%20returning?))
        (if (Variables|Default|GetIs%20the%20elevator%20at%20the%20top?)
          (Variables|Default|SetIs%20the%20elevator%20at%20the%20top? false)
          (bind (_direction _0_1) (Timeline|Animate%20Up/Down ReverseFromEnd)
            (:Update
              (Transformation|SetRelativeLocation (Variables|Default|GetElevator_FloorHinge) (Math|Vector|Lerp(Vector) "0, 0, 0" (Variables|Default|GetElevator%20Height) _0_1) false true))
            (:Finished
              (switch Utilities|FlowControl|Switch|SwitchonETimelineDirection _direction
                (:Forward
                  (bind _asbp_button (Utilities|Casting|CastToBP_Button (Variables|/Script/Engine.ChildActorComponent|GetChildActor (Variables|Default|GetButton_Top_BP))))
                  (Default|ReturnMaterialtoDefaultColour _asbp_button)
                  (if (Variables|Variables|GetBottom%20call%20button%20was%20pressed?)
                    (Variables|Variables|SetBottom%20call%20button%20was%20pressed? false)
                    (Variables|Variables|SetIs%20delay%20activated%20before%20returning? true)
                    (Utilities|FlowControl|Delay (Variables|Default|GetFloor%20pause%20time%20before%20returning%20when%20called) :!label _label)
                    (Variables|Variables|SetIs%20delay%20activated%20before%20returning? false)
                    (CallFunction|TriggerElevator)))
                (:Backward
                  (bind _asbp_button_2 (Utilities|Casting|CastToBP_Button (Variables|/Script/Engine.ChildActorComponent|GetChildActor (Variables|Default|GetButton_Bottom_BP))))
                  (Default|ReturnMaterialtoDefaultColour _asbp_button_2)
                  (if (Variables|Variables|GetTop%20call%20button%20was%20pressed?)
                    (Variables|Variables|SetTop%20call%20button%20was%20pressed? false)
                    (Variables|Variables|SetIs%20delay%20activated%20before%20returning? true)
                    (goto _label))))))
          (else
            (Variables|Default|SetIs%20the%20elevator%20at%20the%20top? true)
            (Timeline|Animate%20Up/Down PlayFromStart)))))))

(fn ConstructionScript
  (bind _elevator_floor (Variables|Default|GetElevator_Floor))
  (bind _box (Variables|Default|GetBox))
  (bind _boxextent (Collision|GetComponentBounds _elevator_floor))
  (bind (_min _max) (Components|StaticMesh|GetLocalBounds _elevator_floor))
  (bind _returnvalue (+ _min _max))
  (bind _returnvalue_2 (/ _returnvalue 2.0))
  (Components|StaticMesh|SetStaticMesh (Variables|Default|GetElevator_Floor) (Variables|Default|GetNew%20Elevator%20Floor%20Asset))
  (Components|StaticMesh|SetStaticMesh (Variables|Default|GetElevator_Base) (Variables|Default|GetNew%20Elevator%20Base%20Asset))
  (Components|StaticMesh|SetStaticMesh (Variables|Default|GetElevator_Guide) (Variables|Default|GetNew%20Elevator%20Guide%20Asset))
  (Components|StaticMesh|SetStaticMesh (Variables|Default|GetElevator_FloorHinge) (Variables|Default|GetNew%20Elevator%20Hinge%20Asset))
  (Transformation|SetRelativeTransform (Variables|Default|GetButton_Top_BP) (Variables|Default|GetTop%20%20Button%20Location) false true)
  (Transformation|SetRelativeTransform (Variables|Default|GetButton_Bottom_BP) (Variables|Default|GetBottom%20Button%20Location) false true)
  (Transformation|SetRelativeScale3D _box (Math|Vector|MakeVector (- (.x _boxextent) 1e+01) (- (.y _boxextent) 1e+01) (/ (Variables|Default|GetInteraction%20Box%20Height) 1e+01)))
  (Transformation|SetRelativeLocation _box (Math|Vector|MakeVector (.x _returnvalue_2) (.y _returnvalue_2) (Variables|Default|GetInteraction%20Box%20Height)) false true)
  (Variables|Default|SetElevator%20Height (Math|Vector|MakeVector 0.0 (Math|Float|SelectFloat (.y (Variables|Default|GetElevator%20Height)) 0.0 (< (.y (Variables|Default|GetElevator%20Height)) 0.0)) (.z (Variables|Default|GetElevator%20Height))))
  (Transformation|SetRelativeScale3D (Variables|Default|GetElevator_Guide) (Math|Vector|MakeVector 1.0 1.0 (/ (Math|Vector|VectorLength (Variables|Default|GetElevator%20Height)) 2e+02)))
  (Transformation|SetRelativeLocation (Variables|Default|GetElevator_FloorHinge) (select (Variables|Default|GetIs%20the%20elevator%20at%20the%20top?) (Variables|Default|GetElevator%20Height) "0, 0, 0") false true)
  (Transformation|SetRelativeRotation (Variables|Default|GetElevator_Guide) (Math|Rotator|MakeRotator (- (.pitch (Math|Rotator|FindLookatRotation (Math|Vector|MakeVector 0.0 0.0 0.0) (Variables|Default|GetElevator%20Height))) 9e+01) 0.0 0.0) false true)
  (Transformation|SetRelativeRotation (Variables|Default|GetElevator_Floor) (Math|Rotator|MakeRotator (+ (* (.pitch (Math|Rotator|FindLookatRotation (Math|Vector|MakeVector 0.0 0.0 0.0) (Variables|Default|GetElevator%20Height))) -1.0) 9e+01) 0.0 0.0) false true))
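; BP_Button is a pressable elevator call button, used as a child actor of BP_Elevator.
; A box overlap enables input for the player pawn, so E works only while the player is inside.
; Pressing E sends the button's location tag to the parent elevator, turns it glowing green and plays a timeline press animation that blocks re-presses until finished.
; A custom event, not called within this Blueprint, restores the white material.
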(event OnComponentBeginOverlap(Box)
  (params (OverlappedComponent :type Primitive%20Component%20Object%20Reference) (OtherActor :type Actor%20Object%20Reference) (OtherComp :type Primitive%20Component%20Object%20Reference) (OtherBodyIndex :type Integer) (bFromSweep :type Boolean) (SweepResult :type Hit%20Result%20Structure%20%28by%20ref%29))
  (if (== OtherActor (Game|Player|GetPlayerPawn 0))
    (Input|EnableInput (Game|GetPlayerController 0))))

(event OnComponentEndOverlap(Box)
  (params (OverlappedComponent :type Primitive%20Component%20Object%20Reference) (OtherActor :type Actor%20Object%20Reference) (OtherComp :type Primitive%20Component%20Object%20Reference) (OtherBodyIndex :type Integer))
  (if (== OtherActor (Game|Player|GetPlayerPawn 0))
    (Input|DisableInput (Game|GetPlayerController 0))))

(event Custom|Return%20material%20to%20default%20colour
  (Rendering|Material|SetMaterial (Variables|Default|GetButton) 0 "/Game/Blockout/Material/MInst_PlaneWhite.MInst_PlaneWhite"))

(event Input|KeyboardEvents|E
  (params (Key :type Key%20Structure))
  (:Pressed
    (if (not (Variables|Default|GetWait%20to%20re-activate))
      (Variables|Default|SetWait%20to%20re-activate true)
      (Utilities|FlowControl|Sequence
        (:then_0
          (bind _asbp_elevator (Utilities|Casting|CastToBP_Elevator (Actor|GetParentActor)))
          (Default|CallButtonWasPressed _asbp_elevator (Variables|Default|GetButton%20Location%20Tag)))
        (:then_1
          (Rendering|Material|SetMaterial (Variables|Default|GetButton) 0 "/Game/Blockout/Material/MInst_GlowGreen.MInst_GlowGreen")
          (bind _0_1_0 (Timeline|Animate%20Button PlayFromStart)
            (:Update
              (Transformation|SetRelativeLocation (Variables|Default|GetButton) (Math|Vector|MakeVector 0.0 0.0 (Math|Float|Lerp 0.0 -2.0 _0_1_0)) false true))
            (:Finished
              (Variables|Default|SetWait%20to%20re-activate false))))))))

(fn ConstructionScript)
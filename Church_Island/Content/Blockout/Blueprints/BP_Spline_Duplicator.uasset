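; Construction-script blockout tool that builds meshes along an editable spline, optionally as a closed loop.
; Each segment gets a spline mesh following point tangents, roll and scale, with width/height multipliers, sideways offset and configurable collision.
; Optional static meshes mark every point, and optional caps sit at the first and last points.
; Debug mode applies tinted dynamic materials, world-projected or 2D; otherwise segment and point meshes accept custom materials.
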(event EventBeginPlay)

(event Collision|EventActorBeginOverlap
  (params (OtherActor :type Actor%20Object%20Reference)))

(event EventTick
  (params (DeltaSeconds :type Float%20%28single-precision%29)))

(fn ConstructionScript
  (bind _spline (Variables|Default|GetSpline))
  (bind _custom_spline_point_asset_material (Variables|Material|GetCustom%20Spline%20Point%20Asset%20Material))
  (bind _custom_spline_asset_material (Variables|Material|GetCustom%20Spline%20Asset%20Material))
  (bind _is_closed_loop_ (Variables|Default|GetIs%20Closed%20Loop?))
  (bind _use_world_projected_texture_ (Variables|Material|GetUse%20World%20Projected%20Texture?))
  (bind _spline_2 (Variables|Default|GetSpline))
  (bind _tangent_point_offsets (Variables|Default|GetTangent%20Point%20Offsets))
  (bind _spline_3 (Variables|Default|GetSpline))
  (bind _spline_4 (Variables|Default|GetSpline))
  (bind _height_multiply (Variables|Default|GetHeight%20Multiply))
  (bind _width_multiply (Variables|Default|GetWidth%20Multiply))
  (bind _spline_5 (Variables|Default|GetSpline))
  (bind _spline_6 (Variables|Default|GetSpline))
  (bind _spline_7 (Variables|Default|GetSpline))
  (bind _spline_8 (Variables|Default|GetSpline))
  (bind _offset_left_right (Variables|Default|GetOffset%20Left-Right))
  (bind _returnvalue (Spline|GetScaleatSplinePoint _spline_6 0))
  (bind _returnvalue_2 (Spline|GetNumberOfSplinePoints _spline_7))
  (bind _returnvalue_3 (Math|Integer|SelectInt 0 1 _is_closed_loop_))
  (bind _returnvalue_4 (Spline|GetNumberOfSplinePoints _spline_2))
  (bind _returnvalue_5 (select _use_world_projected_texture_ "/Game/Blockout/Material/Base/M_WorldProject.M_WorldProject" "/Game/Blockout/Material/MInst_2D.MInst_2D"))
  (bind _returnvalue_6 (- _returnvalue_2 1))
  (bind _returnvalue_7 (- _returnvalue_4 _returnvalue_3))
  (bind _returnvalue_8 (Spline|GetScaleatSplinePoint _spline _returnvalue_6))
  (Utilities|Array|Clear (Variables|Variables|GetCreated%20Assets%20%28Reference%29))
  (Spline|SetClosedLoop (Variables|Default|GetSpline) (Variables|Default|GetIs%20Closed%20Loop?) true)
  (if (Variables|Material|GetUse%20Debug%20Material?)
    (bind _returnvalue_9 (Rendering|Material|CreateDynamicMaterialInstance _returnvalue_5 "None" :!class /Script/Engine.KismetMaterialLibrary))
    (bind _output_get (Variables|Variables|SetSpline%20Mesh%20Dynamic%20Material _returnvalue_9))
    (Rendering|Material|SetVectorParameterValue _output_get "Diffuse Colour" (Variables|Material|GetSurface%20Colour) :!class /Script/Engine.MaterialInstanceDynamic)
    (Rendering|Material|SetScalarParameterValue _output_get "Unique colour for top?" (Math|Conversions|ToFloat(Boolean) (Variables|Material|GetUnique%20colour%20for%20top?)) :!class /Script/Engine.MaterialInstanceDynamic)
    (Rendering|Material|SetVectorParameterValue _output_get "Diffuse Colour - Top" (Variables|Material|GetTop%20Colour) :!class /Script/Engine.MaterialInstanceDynamic)
    (Rendering|Material|SetScalarParameterValue _output_get "Roughness" (Variables|Material|GetMaterial%20Roughness%20Value) :!class /Script/Engine.MaterialInstanceDynamic)
    (bind _returnvalue_10 (Rendering|Material|CreateDynamicMaterialInstance _returnvalue_5 "None" :!class /Script/Engine.KismetMaterialLibrary))
    (bind _output_get_2 (Variables|Variables|SetSpline%20Point/End%20Dynamic%20Material _returnvalue_10))
    (Rendering|Material|SetVectorParameterValue _output_get_2 "Diffuse Colour" (Variables|Default|GetSpline%20Point%20Asset%20Colour) :!class /Script/Engine.MaterialInstanceDynamic)
    (Rendering|Material|SetScalarParameterValue _output_get_2 "Unique colour for top?" (Math|Conversions|ToFloat(Boolean) (Variables|Material|GetUnique%20colour%20for%20top?)) :!class /Script/Engine.MaterialInstanceDynamic)
    (Rendering|Material|SetVectorParameterValue _output_get_2 "Diffuse Colour - Top" (Variables|Material|GetTop%20Colour) :!class /Script/Engine.MaterialInstanceDynamic)
    (Rendering|Material|SetScalarParameterValue _output_get_2 "Roughness" (Variables|Material|GetMaterial%20Roughness%20Value) :!class /Script/Engine.MaterialInstanceDynamic))
  (for _index (range 0 _returnvalue_7)
    (Utilities|IsValid (Variables|Default|GetNew%20Spline%20Point%20Asset)
      (:Is%20Valid
        (bind _returnvalue_11 (AddComponent|AddStaticMeshComponent false (Math|Transform|MakeTransform (Spline|GetLocationatSplinePoint _spline_8 _index "Local") (Math|Conversions|RotationFromXVector (Spline|GetTangentatSplinePoint _spline_8 _index "Local")) (Math|Vector|MakeVector 1.0 1.0 (* (.z (Spline|GetScaleatSplinePoint (Variables|Default|GetSpline) _index)) (Variables|Default|GetHeight%20Multiply))))))
        (Components|StaticMesh|SetStaticMesh _returnvalue_11 (Variables|Default|GetNew%20Spline%20Point%20Asset))
        (Transformation|AddLocalRotation _returnvalue_11 (Math|Rotator|MakeRotator (+ (Variables|Default|GetSpline%20Point%20Asset%20-%20Rotation) (Spline|GetRollatSplinePoint (Variables|Default|GetSpline) _index "Local")) 0.0 0.0) false true)
        (Transformation|AddLocalOffset _returnvalue_11 (Math|Vector|MakeVector 0.0 (Variables|Default|GetOffset%20Left-Right) 0.0) false true)
        (if (Variables|Material|GetUse%20Debug%20Material?)
          (Rendering|Material|SetMaterial _returnvalue_11 0 (Variables|Variables|GetSpline%20Point/End%20Dynamic%20Material))
          (else
            (Utilities|IsValid _custom_spline_point_asset_material
              (:Is%20Valid
                (Rendering|Material|SetMaterial _returnvalue_11 (Variables|Material|GetCustom%20Spline%20Point%20Asset%20Material%20ID) _custom_spline_point_asset_material))
              (:Is%20Not%20Valid
                _)))))
      (:Is%20Not%20Valid
        _))
    (if (not (== _index _returnvalue_7))
      (bind _returnvalue_12 (AddComponent|AddSplineMeshComponent false))
      (Utilities|Array|Add (Variables|Variables|GetCreated%20Assets%20%28Reference%29) _returnvalue_12)
      (SplineMesh|SetForwardAxis _returnvalue_12 (Variables|Default|GetForward%20Axis) false)
      (SplineMesh|SetSplineUpDir _returnvalue_12 (Variables|Default|GetSpline%20Up%20Direction) false)
      (Collision|SetCollisionEnabled _returnvalue_12 (select (Variables|Default|GetDisable%20Collision?) "NoCollision" "QueryAndPhysics"))
      (Collision|SetCollisionResponsetoChannel _returnvalue_12 "ECC_Camera" (Variables|Default|GetCamera%20Interaction))
      (Components|StaticMesh|SetStaticMesh _returnvalue_12 (Variables|Default|GetNew%20Spline%20Asset))
      (if (Variables|Material|GetUse%20Debug%20Material?)
        (Rendering|Material|SetMaterial _returnvalue_12 0 (Variables|Variables|GetSpline%20Mesh%20Dynamic%20Material))
        (else
          (Utilities|IsValid _custom_spline_asset_material
            (:Is%20Valid
              (Rendering|Material|SetMaterial _returnvalue_12 (Variables|Material|GetCustom%20Spline%20Asset%20Material%20ID) _custom_spline_asset_material))
            (:Is%20Not%20Valid
              _))))
      (SplineMesh|SetStartandEnd _returnvalue_12 (+ (* (Class|SplineComponent|GetRightVectoratSplinePoint _spline_5 _index "Local") _offset_left_right) (.Location (Spline|GetLocationandTangentatSplinePoint _spline_5 _index "Local"))) (+ _tangent_point_offsets (.Tangent (Spline|GetLocationandTangentatSplinePoint _spline_5 _index "Local"))) (+ (* (Class|SplineComponent|GetRightVectoratSplinePoint _spline_5 (+ _index 1) "Local") _offset_left_right) (.Location (Spline|GetLocationandTangentatSplinePoint (Variables|Default|GetSpline) (+ _index 1) "Local"))) (+ _tangent_point_offsets (.Tangent (Spline|GetLocationandTangentatSplinePoint (Variables|Default|GetSpline) (+ _index 1) "Local"))) false :!class /Script/Engine.SplineMeshComponent)
      (Class|SplineMeshComponent|SetStartRoll _returnvalue_12 (/ (Spline|GetRollatSplinePoint _spline_3 _index "Local") 56.5) false)
      (Class|SplineMeshComponent|SetEndRoll _returnvalue_12 (/ (Spline|GetRollatSplinePoint _spline_3 (+ _index 1) "Local") 56.5) false)
      (SplineMesh|SetStartScale _returnvalue_12 (Math|Vector2D|MakeVector2D (* _width_multiply (.y (Spline|GetScaleatSplinePoint _spline_4 _index))) (* _height_multiply (.z (Spline|GetScaleatSplinePoint _spline_4 _index)))) false :!class /Script/Engine.SplineMeshComponent)
      (SplineMesh|SetEndScale _returnvalue_12 (Math|Vector2D|MakeVector2D (* _width_multiply (.y (Spline|GetScaleatSplinePoint _spline_4 (+ _index 1)))) (* _height_multiply (.z (Spline|GetScaleatSplinePoint _spline_4 (+ _index 1))))) true :!class /Script/Engine.SplineMeshComponent)))
  (Utilities|FlowControl|Sequence
    (:then_0
      (Utilities|IsValid (Variables|Default|GetNew%20Start%20Cap%20Asset)
        (:Is%20Valid
          (bind _returnvalue_13 (AddComponent|AddStaticMeshComponent false (Math|Transform|MakeTransform (Spline|GetLocationatSplinePoint _spline_6 0 "Local") (Math|Conversions|RotationFromXVector (Spline|GetTangentatSplinePoint _spline_6 0 "Local")) (Math|Vector|MakeVector 1.0 (* (.y _returnvalue) (Variables|Default|GetWidth%20Multiply)) (* (.z _returnvalue) (Variables|Default|GetHeight%20Multiply))))))
          (Components|StaticMesh|SetStaticMesh _returnvalue_13 (Variables|Default|GetNew%20Start%20Cap%20Asset))
          (Transformation|AddRelativeRotation _returnvalue_13 "0,180.000000, 0" false false)
          (if (Variables|Material|GetUse%20Debug%20Material?)
            (Rendering|Material|SetMaterial _returnvalue_13 0 (Variables|Variables|GetSpline%20Point/End%20Dynamic%20Material))))))
    (:then_1
      (Utilities|IsValid (Variables|Default|GetNew%20End%20Cap%20Asset)
        (:Is%20Valid
          (bind _returnvalue_14 (AddComponent|AddStaticMeshComponent false (Math|Transform|MakeTransform (Spline|GetLocationatSplinePoint _spline _returnvalue_6 "Local") (Math|Conversions|RotationFromXVector (Spline|GetTangentatSplinePoint _spline _returnvalue_6 "Local")) (Math|Vector|MakeVector 1.0 (* (.y _returnvalue_8) (Variables|Default|GetWidth%20Multiply)) (* (.z _returnvalue_8) (Variables|Default|GetHeight%20Multiply))))))
          (Components|StaticMesh|SetStaticMesh _returnvalue_14 (Variables|Default|GetNew%20End%20Cap%20Asset))
          (if (Variables|Material|GetUse%20Debug%20Material?)
            (Rendering|Material|SetMaterial _returnvalue_14 0 (Variables|Variables|GetSpline%20Point/End%20Dynamic%20Material))))))))
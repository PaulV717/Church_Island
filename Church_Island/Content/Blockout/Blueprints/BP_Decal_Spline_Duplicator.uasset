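; Blockout spline tool that spawns decal components along an editable, optionally looped spline in the construction script.
; Decals are placed by fixed spacing or count, following the full spline tangent or only its yaw.
; Primary and optional secondary material, scale and offsets alternate via FlipFlop, with an option to pick materials randomly from an array.
; Unseeded random location, rotation and added scale re-roll on each reconstruction.
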(event EventBeginPlay)

(event Collision|EventActorBeginOverlap
  (params (OtherActor :type Actor%20Object%20Reference)))

(event EventTick
  (params (DeltaSeconds :type Float%20%28single-precision%29)))

(fn ConstructionScript
  (bind _spline (Variables|Default|GetSpline))
  (bind _rotation_randomization_strength (Variables|Default|GetRotation%20Randomization%20Strength))
  (bind _location_randomization_strength (Variables|Default|GetLocation%20Randomization%20Strength))
  (bind _count_per_spline (Variables|Default|GetCount%20per%20spline))
  (bind _secondary_decal___material (Variables|Materials|GetSecondary%20Decal%20-%20Material))
  (bind _randomized_material_array (Variables|Materials|GetRandomized%20Material%20Array))
  (bind _scale_randomization_strength (Variables|Default|GetScale%20Randomization%20Strength))
  (bind _returnvalue (Utilities|Array|Length _randomized_material_array))
  (Spline|SetClosedLoop (Variables|Default|GetSpline) (Variables|Default|GetIs%20Closed%20loop?) true)
  (Variables|Variables|SetSpline%20Length (Spline|GetSplineLength (Variables|Default|GetSpline)))
  (for _index (range 0 (select (Variables|Default|GetT=Spacing%20F=Count%20per%20spline) (Math|Float|Floor (/ (Variables|Variables|GetSpline%20Length) (Variables|Default|GetDecal%20Spacing))) (- (Variables|Default|GetCount%20per%20spline) 1)))
    (bind _isa (Utilities|FlowControl|FlipFlop)
      (:A
        _)
      (:B
        _))
    (bind _returnvalue_2 (AddComponent|AddDecalComponent false (Math|Transform|MakeTransform (Spline|GetLocationatDistanceAlongSpline _spline (* _index (select (Variables|Default|GetT=Spacing%20F=Count%20per%20spline) (Variables|Default|GetDecal%20Spacing) (/ (Variables|Variables|GetSpline%20Length) (Math|Conversions|ToFloat(Integer) (select (Variables|Default|GetIs%20Closed%20loop?) (- _count_per_spline 0) (- _count_per_spline 1)))))) "Local") (select (Variables|Default|GetAlign%20to%20splines%20orientation?) (Math|Conversions|RotationFromXVector (Spline|GetTangentatDistanceAlongSpline _spline (* _index (select (Variables|Default|GetT=Spacing%20F=Count%20per%20spline) (Variables|Default|GetDecal%20Spacing) (/ (Variables|Variables|GetSpline%20Length) (Math|Conversions|ToFloat(Integer) (select (Variables|Default|GetIs%20Closed%20loop?) (- _count_per_spline 0) (- _count_per_spline 1)))))) "Local")) (Math|Rotator|MakeRotator 1.8e+02 0.0 (.Yaw (Math|Rotator|BreakRotator (Math|Conversions|RotationFromXVector (Spline|GetTangentatDistanceAlongSpline _spline (* _index (select (Variables|Default|GetT=Spacing%20F=Count%20per%20spline) (Variables|Default|GetDecal%20Spacing) (/ (Variables|Variables|GetSpline%20Length) (Math|Conversions|ToFloat(Integer) (select (Variables|Default|GetIs%20Closed%20loop?) (- _count_per_spline 0) (- _count_per_spline 1)))))) "Local")))))) (+ (Math|Vector|MakeVector (Math|Random|RandomFloatinRange 0.0 (.x _scale_randomization_strength)) (Math|Random|RandomFloatinRange 0.0 (.y _scale_randomization_strength)) (Math|Random|RandomFloatinRange 0.0 (.z _scale_randomization_strength))) (select (and (Utilities|IsValid (Variables|Materials|GetSecondary%20Decal%20-%20Material)) _isa) (Variables|Materials|GetSecondary%20Decal%20-%20Scale) (Variables|Materials|GetPrimary%20Decal%20-%20Scale))))))
    (Rendering|Components|Decal|SetDecalMaterial _returnvalue_2 (select (Variables|Materials|GetRandomize%20Material%20?) (select (== _returnvalue 0) (select (and (Utilities|IsValid _secondary_decal___material) _isa) _secondary_decal___material (Variables|Materials|GetPrimary%20Decal%20-%20Material)) (Utilities|Array|Get(acopy) (Variables|Materials|GetRandomized%20Material%20Array) (Math|Random|RandomIntegerinRange 0 (- _returnvalue 1)))) (select (and (Utilities|IsValid _secondary_decal___material) _isa) _secondary_decal___material (Variables|Materials|GetPrimary%20Decal%20-%20Material))))
    (Transformation|AddLocalOffset _returnvalue_2 (select (and (Utilities|IsValid (Variables|Materials|GetSecondary%20Decal%20-%20Material)) _isa) (Variables|Materials|GetSecondary%20Decal%20-%20Local%20Location%20Offset) (Variables|Materials|GetPrimary%20Decal%20-%20Local%20Location%20Offset)) false false)
    (Transformation|AddLocalOffset _returnvalue_2 (Math|Vector|MakeVector (Math|Random|RandomFloatinRange (* (.x _location_randomization_strength) -1.0) (.x _location_randomization_strength)) (Math|Random|RandomFloatinRange (* (.y _location_randomization_strength) -1.0) (.y _location_randomization_strength)) (Math|Random|RandomFloatinRange (* (.z _location_randomization_strength) -1.0) (.z _location_randomization_strength))) false false)
    (Transformation|AddLocalRotation _returnvalue_2 (select (Variables|Default|GetAlign%20to%20splines%20orientation?) (Math|Rotator|CombineRotators (Math|Rotator|CombineRotators (select (and (Utilities|IsValid (Variables|Materials|GetSecondary%20Decal%20-%20Material)) _isa) (Variables|Materials|GetSecondary%20Decal%20-%20%20Local%20rotation%20Offset) (Variables|Materials|GetPrimary%20Decal%20-%20%20Local%20rotation%20Offset)) (Math|Rotator|MakeRotator 0.0 9e+01 (Variables|Default|GetGlobal%20Rotation))) "0, 0,180.000000") (Math|Rotator|CombineRotators (select (and (Utilities|IsValid (Variables|Materials|GetSecondary%20Decal%20-%20Material)) _isa) (Variables|Materials|GetSecondary%20Decal%20-%20%20Local%20rotation%20Offset) (Variables|Materials|GetPrimary%20Decal%20-%20%20Local%20rotation%20Offset)) (Math|Rotator|MakeRotator 0.0 9e+01 (Variables|Default|GetGlobal%20Rotation)))) false false)
    (Transformation|AddLocalRotation _returnvalue_2 (Math|Rotator|MakeRotator (Math|Random|RandomFloatinRange (* (.roll _rotation_randomization_strength) -1.0) (.roll _rotation_randomization_strength)) (Math|Random|RandomFloatinRange (* (.pitch _rotation_randomization_strength) -1.0) (.pitch _rotation_randomization_strength)) (Math|Random|RandomFloatinRange (* (.yaw _rotation_randomization_strength) -1.0) (.yaw _rotation_randomization_strength))) false false)
    (Class|DecalComponent|SetSortOrder _returnvalue_2 (Variables|Default|GetSort%20Order))
    (Rendering|Components|Decal|SetFadeScreenSize _returnvalue_2 (Variables|Default|GetFade%20Screen%20Size))))